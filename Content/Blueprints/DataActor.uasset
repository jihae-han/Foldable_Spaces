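; DataActor logs walking-test data as CSV rows of ID, walking time, distance and collision count.
; Pressing F1 appends a row to an in-memory array and prints it, with real-time seconds as walking time and distance and collisions fixed at zero.
; EndPlay adds a final row through the same path, then saves the array to a timestamped .csv in the project's Data folder.
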(event `self.ReceiveBeginPlay`)

(event `Key|F1`
  (params (Key :type "Key Structure"))
  (bind _testarray (`self.TestArray`))
  (bind (_datastruct_walkingtime _datastruct_walkingdistance _datastruct_collisioncount) (break `/Game/Blueprints/DataStruct` (make `/Game/Blueprints/DataStruct` (`GameplayStatics.GetRealTimeSeconds`))))
  (:`Pressed`
    (bind _output_get (set `self.TestRow` (`KismetStringLibrary.Concat_StrStr` (`self.ID`) "," (`KismetStringLibrary.Conv_DoubleToString` _datastruct_walkingtime) "," (`KismetStringLibrary.Conv_DoubleToString` _datastruct_walkingdistance) "," (`KismetStringLibrary.Conv_IntToString` _datastruct_collisioncount)) :!label _label))
    (`KismetArrayLibrary.Array_Add` _testarray _output_get)
    (`KismetSystemLibrary.PrintString` (`|GetArrayItem` _testarray (- (`KismetArrayLibrary.Array_Length` _testarray) 1)))))

(event `self.ReceiveEndPlay`
  (params (EndPlayReason :type "EEndPlayReason Enum" :default "Destroyed"))
  (bind (_returnvalue_year _returnvalue_month _returnvalue_day _returnvalue_hour _returnvalue_minute _returnvalue_second) (`KismetMathLibrary.BreakDateTime` (`KismetMathLibrary.Now`)))
  (`|ExecutionSequence`
    (:`then_0`
      (goto _label))
    (:`then_1`
      (`MyTextFileManager.SaveArrayText` (`KismetStringLibrary.Concat_StrStr` (`KismetSystemLibrary.GetProjectDirectory`) "/Data") (`KismetStringLibrary.Concat_StrStr` (`KismetStringLibrary.Conv_IntToString` _returnvalue_year) "." (`KismetStringLibrary.Conv_IntToString` _returnvalue_month) "." (`KismetStringLibrary.Conv_IntToString` _returnvalue_day) "_" (`KismetStringLibrary.Conv_IntToString` _returnvalue_hour) "." (`KismetStringLibrary.Conv_IntToString` _returnvalue_minute) "." (`KismetStringLibrary.Conv_IntToString` _returnvalue_second) ".csv") (`self.TestArray`)))))

(fn `UserConstructionScript`)