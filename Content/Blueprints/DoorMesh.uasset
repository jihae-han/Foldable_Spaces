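; DoorMesh builds a procedural wall with a door opening, themed by its Type.
; The construction script places the opening from DoorPosition, builds two mesh sections with opposite triangle winding and separate materials, and sizes an overlap box to the wall.
; SpawnContent sets the first mesh's material by Type, then spawns and attaches a Fill actor given that box and Type.
; The TwoSided branch is empty on both sides.
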(event `/Game/Blueprints/DoorMeshInterface.SpawnContent`
  (bind _proceduralmesh (`self.ProceduralMesh`))
  ;[0 0 0] ContentSpawner
  (`|ExecutionSequence`
    (:`then_0`
      (switch `/Game/Blueprints/PageEnum` (`self.Type`)
        (:`NewEnumerator0`
          (`PrimitiveComponent.SetMaterial` _proceduralmesh 0 "/Game/Floor/M_Ground_Grass.M_Ground_Grass"))
        (:`NewEnumerator1`
          (`PrimitiveComponent.SetMaterial` _proceduralmesh 0 "/Game/Imports/Seaside_Town/Materials/Tilables/MI_Floors_Stone_Inst4.MI_Floors_Stone_Inst4"))
        (:`NewEnumerator2`
          (`PrimitiveComponent.SetMaterial` _proceduralmesh 0 "/Game/Floor/M_URockB.M_URockB"))
        (:`NewEnumerator3`
          (`PrimitiveComponent.SetMaterial` _proceduralmesh 0 "/Game/Imports/FreeFurniturePack/Materials/M_Chrome.M_Chrome"))
        (:`NewEnumerator4`
          (`PrimitiveComponent.SetMaterial` _proceduralmesh 0 "/Game/Floor/M_Basic_Wall.M_Basic_Wall"))
        (:`NewEnumerator5`
          (`PrimitiveComponent.SetMaterial` _proceduralmesh 0 "/Game/Floor/M_Wood_Floor_Walnut_Polished.M_Wood_Floor_Walnut_Polished"))
        (:`NewEnumerator6`
          (`PrimitiveComponent.SetMaterialByName` _proceduralmesh "None" "/Game/Imports/ModernCityEnvironment01/Materials/M_MMetro_Floor.M_MMetro_Floor"))))
    (:`then_1`
      (bind _returnvalue (`|SpawnActorFromClass` "/Game/Blueprints/Fill.Fill_C" (`KismetMathLibrary.MakeTransform` (0.0 0.0 0.0)) "AlwaysSpawn" "OverrideRootScale" null (`self.Overlapping`) (`self.Type`) 0.0 0.0 0.0 null))
      (`self.K2_AttachToComponent` _returnvalue (`self.ProceduralMesh`) "None" "KeepRelative" "KeepRelative" "KeepRelative" true))))

(fn `UserConstructionScript`
  (bind _array (`|MakeArray` (0.0 0.0) (0.0 1.0) (0.5 1.0) (1.0 1.0) (1.0 0.0) (0.6 0.0) (0.6 0.8) (0.3 0.8) (0.3 0.0) :!type "Vector2D Structure"))
  (bind _overlapping (`self.Overlapping`))
  (bind _doorposition_ (`self.DoorPosition%`))
  (bind _doorrightpt (`self.DoorRightPt`))
  (bind _doorleftpt (`self.DoorLeftPt`))
  (bind _proceduralmesh (`self.ProceduralMesh`))
  (bind _doorwidth (`self.DoorWidth`))
  (bind _proceduralmesh_2 (`self.ProceduralMesh`))
  (bind _height (`self.Height`))
  (bind _proceduralmesh1 (`self.ProceduralMesh1`))
  (bind _width (`self.Width`))
  (bind _doorheight (`self.DoorHeight`))
  (bind _returnvalue (/ (`self.Height`) 2.0))
  (bind _returnvalue_2 (/ (`self.Width`) 2.0))
  (bind _returnvalue_3 (* (`self.Width`) _doorposition_))
  (bind _array_2 (`|MakeArray` (0.0 0.0 0.0) (`KismetMathLibrary.MakeVector` 0.0 _height) (`KismetMathLibrary.MakeVector` (/ _width 2.0) _height) (`KismetMathLibrary.MakeVector` _width _height) (`KismetMathLibrary.MakeVector` _width) (`KismetMathLibrary.MakeVector` _doorrightpt) (`KismetMathLibrary.MakeVector` _doorrightpt _doorheight) (`KismetMathLibrary.MakeVector` _doorleftpt _doorheight) (`KismetMathLibrary.MakeVector` _doorleftpt) :!type "Vector Structure"))
  (`|ExecutionSequence`
    (:`then_0`
      ;[0 0 0] SetUp DoorPosition
      (if (> _doorposition_ 0.5)
        (bind _output_get (set `self.DoorRightPt` _returnvalue_3)) ; Door located right
        (set `self.DoorLeftPt` (- _output_get _doorwidth))
        (elif (== (`self.DoorPosition%`) 0.5)
          (bind _output_get_2 (set `self.DoorLeftPt` (- _returnvalue_3 (/ _doorwidth 2.0)))) ; Door  located at midpt?
          (set `self.DoorRightPt` (+ _doorwidth _output_get_2))
          (else
            (bind _output_get_3 (set `self.DoorLeftPt` _returnvalue_3)) ; Door located towards the left
            (set `self.DoorRightPt` (+ _output_get_3 _doorwidth))))))
    (:`then_1`
      ;[0 0 0] Make ProceduralMesh
      (if (`self.TwoSided`)
        _
        (else
          _))
      (`ProceduralMeshComponent.CreateMeshSection_LinearColor` :`self` _proceduralmesh_2 :`Vertices` _array_2 :`Triangles` (`|MakeArray` 0 7 8 0 1 7 1 2 7 7 2 6 6 2 3 3 4 6 4 5 6) :`UV0` _array :`bCreateCollision` true)
      (`PrimitiveComponent.SetMaterial` _proceduralmesh_2 0 (`self.Material`))
      ;[0 0 0] Make ProceduralMesh
      (`|ExecutionSequence`
        (:`then_0`
          (set `self.vertices` _array_2)
          (for (_ _array_index) _array
            (`KismetArrayLibrary.Array_Add` (`self.UV`) (`|GetArrayItem` _array (- (`KismetArrayLibrary.Array_LastIndex` _array) _array_index)))))
        (:`then_1`
          (set `self.triangles` (`|MakeArray` 0 8 7 0 7 1 1 7 2 7 6 2 6 3 2 3 6 4 4 6 5))
          (`ProceduralMeshComponent.CreateMeshSection_LinearColor` :`self` _proceduralmesh1 :`Vertices` (`self.vertices`) :`Triangles` (`self.triangles`) :`UV0` (`self.UV`) :`bCreateCollision` true)
          (`PrimitiveComponent.SetMaterial` _proceduralmesh1 0 (`self.Material1`)))))
    (:`then_2`
      ;[0 0 0] overlapping Collision
      (`BoxComponent.SetBoxExtent` _overlapping (`KismetMathLibrary.MakeVector` _returnvalue_2 _returnvalue 2.5) true)
      (`SceneComponent.K2_SetRelativeLocation` _overlapping (`KismetMathLibrary.MakeVector` _returnvalue_2 _returnvalue) false false)
      (`SceneComponent.K2_AttachToComponent` (`self.Overlapping`) _proceduralmesh "None" "KeepRelative" "KeepRelative" "KeepRelative" true)
      (`SceneComponent.K2_AttachToComponent` (`self.ProceduralMesh1`) _proceduralmesh "None" "KeepRelative" "KeepRelative" "KeepRelative" true))))