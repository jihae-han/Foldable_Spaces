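; Door is a procedural panel with up to two doorway cutouts that rotates as the VR pawn passes through, switching scenes.
; The construction script builds two meshes, doorway triggers and four edge markers.
; Trigger overlaps compare pawn direction and side to play or reverse roll timelines, attaching pickups and marker-detected neighboring Doors to move along.
; Overlaps and finished rotations message the player controller about scene changes; finishing also detaches Doors.
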(event `self.ReceiveTick`
  (params (DeltaSeconds :type "Float (single-precision)")))

(event `self.ReceiveBeginPlay`
  ;[0 0 0] BeginPlay
)

(event `Attach`
  (params (Parent :type "SceneComponent Object Reference"))
  ;[0 0 0] AttachDoor
  (`self.K2_AttachToComponent` Parent "None" "KeepWorld" "KeepWorld" "KeepWorld"))

(event `Detach`
  ;[0 0 0] AttachDoor
  (`self.K2_DetachFromActor` "KeepWorld" "KeepWorld" "KeepWorld"))

(event `/Game/Blueprints/DoorInterface.Open`
  ;[0 0 0] Door Collision 1 : A
  (`self.AttachDoor`)
  (bind (_direction _90) (`Timeline|Timeline_0` :!label _label)
    (:`Update`
      (`SceneComponent.K2_SetRelativeRotation` (`self.ProceduralMesh`) (`KismetMathLibrary.MakeRotator` (* _90 (`self.Angle`))) false false))
    (:`Finished`
      (`self.DetachDoor` :!label _label_2)
      (`self.SceneControl` (`self.DoorCollision1`)))))

(event `/Game/Blueprints/DoorInterface.Open2`
  ;[0 0 0] Door Collision 1 : A
  (`self.AttachDoor`)
  (bind (_direction _90) (`Timeline|90_180` :!label _label_3)
    (:`Update`
      (`SceneComponent.K2_SetRelativeRotation` (`self.ProceduralMesh`) (`KismetMathLibrary.MakeRotator` (* _90 (`self.Angle`))) false false))
    (:`Finished`
      (goto _label_2))))

(event `self.DoorCollision1.OnComponentBeginOverlap`
  (params (OverlappedComponent :type "PrimitiveComponent Object Reference") (OtherActor :type "Actor Object Reference") (OtherComp :type "PrimitiveComponent Object Reference") (OtherBodyIndex :type Integer) (bFromSweep :type Boolean) (SweepResult :type "HitResult Structure (by ref)"))
  (bind _proceduralmesh (`self.ProceduralMesh`))
  (bind _doornum1 (`self.DoorNum1`))
  (bind _returnvalue_roll (`KismetMathLibrary.BreakRotator` (`SceneComponent.K2_GetComponentRotation` (`self.ProceduralMesh`))))
  (bind (_returnvalue_roll_2 _returnvalue_pitch _returnvalue_yaw) (`KismetMathLibrary.BreakRotator` (`SceneComponent.K2_GetComponentRotation` _proceduralmesh)))
  (bind _returnvalue (< (`KismetMathLibrary.Abs` _returnvalue_roll) 90.0))
  ;[0 0 0] Door Collision 1 : A
  (bind _door (`self.Door_D`))
  (message `/Game/Blueprints/StoryInterface.ChangeScene` (`GameplayStatics.GetPlayerController` 0) "A" (`SceneComponent.K2_GetComponentLocation` _proceduralmesh) _returnvalue_yaw _door)
  (bind _asvr_pawn (cast `/Game/Blueprints/VR_Pawn` OtherActor))
  (`|ExecutionSequence`
    (:`then_0`
      (`self.AttachActors`))
    (:`then_1`
      (`self.AttachDoor`)
      (if (> (`self.DoorNum`) _doornum1)
        (if true
          (`self.CalculateMeshPts` _doornum1)
          (`ProceduralMeshComponent.CreateMeshSection_LinearColor` :`self` (`self.ProceduralMesh1`) :`Vertices` (`self.vertices`) :`Triangles` (`self.triangles`) :`UV0` (`self.UV`) :`bCreateCollision` true)
          (message `/Game/Blueprints/StoryInterface.BranchScene` (`GameplayStatics.GetPlayerController` 0) true "A" self))))
    (:`then_2`
      (bind (_direction _location) (`self.GetPlayerOrientation` _asvr_pawn (`self.DoorCollision1`)))
      (if (and _direction _location _returnvalue)
        (goto _label)
        (elif (and (not _direction) (not _location) (not _returnvalue))
          (goto _label_3 :!via `Reverse`))))))

(event `/Game/Blueprints/DoorInterface.Close1`
  ;[0 0 0] Door Collision 1 : A
  (`self.AttachDoor`)
  (goto _label_3 :!via `Reverse`))

(event `self.DoorCollision1.OnComponentEndOverlap`
  (params (OverlappedComponent :type "PrimitiveComponent Object Reference") (OtherActor :type "Actor Object Reference") (OtherComp :type "PrimitiveComponent Object Reference") (OtherBodyIndex :type Integer))
  ;[0 0 0] Door Collision 1 : A
  (bind _asvr_pawn (cast `/Game/Blueprints/VR_Pawn` OtherActor))
  (`|ExecutionSequence`
    (:`then_0`
      (`self.AttachActors`))
    (:`then_1`
      (bind (_direction _location) (`self.GetPlayerOrientation` _asvr_pawn (`self.DoorCollision1`)))
      (if (and (not _direction) _location)
        (set `self.Clockwise` true)
        (goto _label :!via `Reverse`)
        (elif (and _direction (not _location))
          (set `self.Clockwise` false)
          (goto _label_3))))
    (:`then_2`
      (`self.AttachDoor`))))

(event `self.DoorCollision2.OnComponentBeginOverlap`
  (params (OverlappedComponent :type "PrimitiveComponent Object Reference") (OtherActor :type "Actor Object Reference") (OtherComp :type "PrimitiveComponent Object Reference") (OtherBodyIndex :type Integer) (bFromSweep :type Boolean) (SweepResult :type "HitResult Structure (by ref)"))
  (bind _proceduralmesh (`self.ProceduralMesh`))
  (bind _doornum1 (`self.DoorNum1`))
  (bind (_returnvalue_roll _returnvalue_pitch _returnvalue_yaw) (`KismetMathLibrary.BreakRotator` (`SceneComponent.K2_GetComponentRotation` _proceduralmesh)))
  (bind _returnvalue_roll_2 (`KismetMathLibrary.BreakRotator` (`SceneComponent.K2_GetComponentRotation` (`self.ProceduralMesh`))))
  (bind _returnvalue (< (`KismetMathLibrary.Abs` _returnvalue_roll_2) 90.0))
  ;[0 0 0] Door Collision 2 : B
  (bind _door (`self.Door_D`))
  (message `/Game/Blueprints/StoryInterface.ChangeScene` (`GameplayStatics.GetPlayerController` 0) "B" (`SceneComponent.K2_GetComponentLocation` _proceduralmesh) _returnvalue_yaw _door)
  (bind _asvr_pawn (cast `/Game/Blueprints/VR_Pawn` OtherActor))
  (`|ExecutionSequence`
    (:`then_0`
      (`self.AttachActors`)
      (`self.AttachDoor`)
      (if (> (`self.DoorNum`) _doornum1)
        (`self.CalculateMeshPts` _doornum1 1)
        (`ProceduralMeshComponent.CreateMeshSection_LinearColor` :`self` (`self.ProceduralMesh1`) :`Vertices` (`self.vertices`) :`Triangles` (`self.triangles`) :`UV0` (`self.UV`) :`bCreateCollision` true)
        (message `/Game/Blueprints/StoryInterface.BranchScene` (`GameplayStatics.GetPlayerController` 0) true "B" self)))
    (:`then_1`
      (bind (_direction _location) (`self.GetPlayerOrientation` _asvr_pawn (`self.DoorCollision2`)))
      (if (and _direction _location _returnvalue)
        (bind (_direction_2 _90) (`Timeline|Timeline_2` :!label _label_4)
          (:`Update`
            (`SceneComponent.K2_SetRelativeRotation` (`self.ProceduralMesh`) (`KismetMathLibrary.MakeRotator` (* _90 (`self.Angle`))) false false))
          (:`Finished`
            (`self.DetachDoor` :!label _label_5)
            (`self.SceneControl` (`self.DoorCollision2`))))
        (elif (and (not _direction) (not _location) (not _returnvalue))
          (bind (_direction_3 _90_2) (`Timeline|Timeline_1` :!via `Reverse` :!label _label_6)
            (:`Update`
              (`SceneComponent.K2_SetRelativeRotation` (`self.ProceduralMesh`) (`KismetMathLibrary.MakeRotator` (* _90_2 (`self.Angle`))) false false))
            (:`Finished`
              (goto _label_5))))))))

(event `self.DoorCollision2.OnComponentEndOverlap`
  (params (OverlappedComponent :type "PrimitiveComponent Object Reference") (OtherActor :type "Actor Object Reference") (OtherComp :type "PrimitiveComponent Object Reference") (OtherBodyIndex :type Integer))
  ;[0 0 0] Door Collision 2 : B
  (bind _asvr_pawn (cast `/Game/Blueprints/VR_Pawn` OtherActor))
  (`|ExecutionSequence`
    (:`then_0`
      (`self.AttachActors`))
    (:`then_1`
      (bind (_direction _location) (`self.GetPlayerOrientation` _asvr_pawn (`self.DoorCollision2`)))
      (if (and (not _direction) _location)
        (set `self.Clockwise` true)
        (goto _label_4 :!via `Reverse`)
        (elif (and _direction (not _location))
          (set `self.Clockwise` false)
          (goto _label_6))))
    (:`then_2`
      (`self.AttachDoor`))))

(fn `AttachActors`
  (for _array_element (`PrimitiveComponent.GetOverlappingActors` (`self.Overlapping`) "/Script/Engine.Actor")
    (if (`KismetSystemLibrary.DoesImplementInterface` _array_element "/Game/Blueprints/PickupActorInterface.PickupActorInterface_C")
      (message `/Game/Blueprints/PickupActorInterface.Pickup` _array_element (`self.ProceduralMesh`)))))

(fn `AttachDoor`
  (locals (OriginalPosition :type "Vector Structure" :default (0.0 0.0 0.0)))
  (bind _d (`self.D`))
  (bind _b (`self.B`))
  (bind _a (`self.A`))
  ;[1 1 1] Find Overlapping Door on Marker
  (for _array_element (`PrimitiveComponent.GetOverlappingComponents` (`self.Overlapping`))
    (if (and (!= (`self.DoorCollision2`) _array_element) (!= _array_element (`self.DoorCollision1`)) (!= _array_element (`self.ProceduralMesh`)) (== (`ActorComponent.GetOwner` _array_element) self))
      (bind _output_get (set `self.CurrentMarker` (`.RightS` (`KismetStringLibrary.Split` (`KismetSystemLibrary.GetDisplayName` _array_element) "."))))
      ;[1 1 1] Depending on Marker, attach 'x' Door
      (switch `string` _output_get
        (:`A`
          (`self.Marker` (`self.A`))
          (bind _output_get_2 (set `local.OriginalPosition` (`SceneComponent.RelativeLocation` _d) :!label _label))
          (`SceneComponent.K2_SetRelativeLocation` _d (`KismetMathLibrary.MakeVector` (/ (`self.Width`) 2.0) 0.0 -50.0) false false)
          (`self.Marker` _d)
          (`SceneComponent.K2_SetRelativeLocation` _d _output_get_2 false false))
        (:`B`
          (`self.Marker` (`self.B`))
          (goto _label))
        (:`C`
          (`self.Marker` (`self.C`))
          (if (`self.Clockwise`)
            (bind _output_get_3 (set `local.OriginalPosition` (`SceneComponent.RelativeLocation` _b)))
            (`SceneComponent.K2_SetRelativeLocation` _b (`KismetMathLibrary.MakeVector` (/ (`self.Width`) 2.0) 50.0) false false)
            (`self.Marker` _b)
            (`SceneComponent.K2_SetRelativeLocation` _b _output_get_3 false false)
            (else
              (bind _output_get_4 (set `local.OriginalPosition` (`SceneComponent.RelativeLocation` _a)))
              (`SceneComponent.K2_SetRelativeLocation` _a (`KismetMathLibrary.MakeVector` (/ (`self.Width`) 2.0) -50.0) false false)
              (`self.Marker` _a)
              (`SceneComponent.K2_SetRelativeLocation` _a _output_get_4 false false))))
        (:`D`
          (`self.Marker` (`self.D`)))))))

(fn `CalculateDoorCollision`
  (params (DoorCollision :type "BoxComponent Object Reference") (DoorNum :type Integer))
  (bind _returnvalue (/ (`self.DoorHeight`) 2.0))
  (`BoxComponent.SetBoxExtent` DoorCollision (`KismetMathLibrary.MakeVector` (/ (`self.DoorWidth`) 5.0) 2.5 _returnvalue) true)
  (`SceneComponent.K2_SetRelativeLocation` DoorCollision (`KismetMathLibrary.MakeVector` (/ (+ (`|GetArrayItem` (`self.DoorLeftPts`) DoorNum) (`|GetArrayItem` (`self.DoorRightPts`) DoorNum)) 2.0) -2.5 _returnvalue) false false))

(fn `CalculateMeshPts`
  (params (Selection :type Integer) (DoorIndex :type Integer))
  (bind _doorheight (`self.DoorHeight`))
  (bind _height (`self.Height`))
  (bind _width (`self.Width`))
  (bind _height_2 (`self.Height`))
  (bind _height_3 (`self.Height`))
  (bind _doorheight_2 (`self.DoorHeight`))
  (bind _width_2 (`self.Width`))
  (bind _width_3 (`self.Width`))
  (bind _doorheight_3 (`self.DoorHeight`))
  (bind _output (`|GetArrayItem` (`self.DoorRightPts`)))
  (bind _output_2 (`|GetArrayItem` (`self.DoorLeftPts`)))
  (bind _output_3 (`|GetArrayItem` (`self.DoorRightPts`) DoorIndex))
  (bind _output_4 (`|GetArrayItem` (`self.DoorLeftPts`) DoorIndex))
  (bind _output_5 (`|GetArrayItem` (`self.DoorRightPts`) 1))
  (bind _output_6 (`|GetArrayItem` (`self.DoorLeftPts`) 1))
  (switch `int` Selection
    (:`0`
      (set `self.vertices` (`|MakeArray` (0.0 0.0 0.0) (`KismetMathLibrary.MakeVector` 0.0 _height_2) (`KismetMathLibrary.MakeVector` _width _height_2) (`KismetMathLibrary.MakeVector` _width) :!type "Vector Structure"))
      (set `self.triangles` (`|MakeArray` 0 1 2 0 2 3))
      (set `self.UV` (`|MakeArray` (0.0 0.0) (0.0 1.0) (1.0 1.0) (1.0 0.0) :!type "Vector2D Structure")))
    (:`1`
      (set `self.vertices` (`|MakeArray` (0.0 0.0 0.0) (`KismetMathLibrary.MakeVector` 0.0 _height_3) (`KismetMathLibrary.MakeVector` (/ _width_3 2.0) _height_3) (`KismetMathLibrary.MakeVector` _width_3 _height_3) (`KismetMathLibrary.MakeVector` _width_3) (`KismetMathLibrary.MakeVector` _output_3) (`KismetMathLibrary.MakeVector` _output_3 _doorheight_2) (`KismetMathLibrary.MakeVector` _output_4 _doorheight_2) (`KismetMathLibrary.MakeVector` _output_4) :!type "Vector Structure"))
      (set `self.triangles` (`|MakeArray` 0 7 8 1 7 0 2 7 1 3 6 2 4 6 3 5 6 4 6 7 2))
      (set `self.UV` (`|MakeArray` (0.0 0.0) (0.0 1.0) (0.5 1.0) (1.0 1.0) (1.0 0.0) (0.6 0.0) (0.6 0.8) (0.3 0.8) (0.3 0.0) :!type "Vector2D Structure")))
    (:`2`
      (set `self.vertices` (`|MakeArray` (0.0 0.0 0.0) (`KismetMathLibrary.MakeVector` 0.0 _height) (`KismetMathLibrary.MakeVector` (/ _width_2 2.0) _height) (`KismetMathLibrary.MakeVector` _width_2 _height) (`KismetMathLibrary.MakeVector` _width_2) (`KismetMathLibrary.MakeVector` _output_5) (`KismetMathLibrary.MakeVector` _output_5 _doorheight_3) (`KismetMathLibrary.MakeVector` _output_6 _doorheight_3) (`KismetMathLibrary.MakeVector` _output_6) (`KismetMathLibrary.MakeVector` _output) (`KismetMathLibrary.MakeVector` _output _doorheight) (`KismetMathLibrary.MakeVector` _output_2 _doorheight) (`KismetMathLibrary.MakeVector` _output_2) :!type "Vector Structure"))
      (set `self.triangles` (`|MakeArray` 0 1 11 1 2 11 2 10 11 3 6 2 4 6 3 5 6 4 6 7 2 7 10 2 8 9 7 9 10 7 10 2 7 11 2 10 12 0 11))
      (set `self.UV` (`|MakeArray` (0.0 0.0) (0.0 1.0) (0.5 1.0) (1.0 1.0) (1.0 0.0) (0.8 0.0) (0.8 0.8) (0.6 0.8) (0.6 0.0) (0.4 0.0) (0.4 0.8) (0.2 0.8) (0.2 0.0) :!type "Vector2D Structure")))))

(fn `DetachDoor`
  (bind _attachedactor (`self.AttachedActor`))
  (for _array_element _attachedactor
    (bind _asdoor (cast `/Game/Blueprints/Door` _array_element))
    (`self.Detach` _asdoor))
  (`KismetArrayLibrary.Array_Clear` _attachedactor))

(fn `Disable`
  (params (`Disable?` :type Boolean) (DoorCollision :type "BoxComponent Object Reference"))
  (bind _returnvalue (not `Disable?`))
  (`self.SetActorHiddenInGame` `Disable?`)
  (`self.SetActorTickEnabled` _returnvalue)
  (`self.SetActorEnableCollision` _returnvalue))

(fn `Door_D`
  (returns (Door :type "/Game/Blueprints/Door Object Reference"))
  (for _array_element (`PrimitiveComponent.GetOverlappingComponents` (`self.D`))
    (bind _returnvalue (`ActorComponent.GetOwner` _array_element))
    (if (!= _returnvalue self)
      (bind _asdoor (cast `/Game/Blueprints/Door` _returnvalue))
      (if (`KismetStringLibrary.Contains` (`KismetSystemLibrary.GetDisplayName` _array_element) "Overlapping")
        (return _asdoor)))))

(fn `Fill`
  (params (Type :type "/Game/Blueprints/PageEnum Enum" :default "NewEnumerator0") (Up :type Boolean :default true))
  (bind _proceduralmesh (`self.ProceduralMesh`))
  (`|ExecutionSequence`
    (:`then_0`
      (switch `/Game/Blueprints/PageEnum` Type
        (:`NewEnumerator0`
          (`PrimitiveComponent.SetMaterial` _proceduralmesh 0 "/Game/StarterContent/Materials/M_Ground_Grass.M_Ground_Grass"))
        (:`NewEnumerator1`
          (`PrimitiveComponent.SetMaterial` _proceduralmesh 0 "/Game/StarterContent/Materials/M_Rock_Sandstone.M_Rock_Sandstone"))
        (:`NewEnumerator2`
          (`PrimitiveComponent.SetMaterial` _proceduralmesh 0 "/Game/Floor/M_URockB.M_URockB"))
        (:`NewEnumerator3`
          (`PrimitiveComponent.SetMaterial` _proceduralmesh 0 "/Game/StarterContent/Materials/M_Metal_Chrome.M_Metal_Chrome"))
        (:`NewEnumerator4`
          (`PrimitiveComponent.SetMaterial` _proceduralmesh 0 "/Game/Floor/M_Basic_Wall.M_Basic_Wall"))
        (:`NewEnumerator5`
          (`PrimitiveComponent.SetMaterial` _proceduralmesh 0 "/Game/Floor/M_Wood_Floor_Walnut_Polished.M_Wood_Floor_Walnut_Polished"))
        (:`NewEnumerator6`
          (`PrimitiveComponent.SetMaterialByName` _proceduralmesh "None" "/Game/VirtualReality/Materials/M_ArcEndpoint.M_ArcEndpoint"))))
    (:`then_1`
      (if Up
        (bind _returnvalue (`|SpawnActorFromClass` "/Game/Blueprints/Fill.Fill_C" (`KismetMathLibrary.MakeTransform` (0.0 0.0 0.0)) "AlwaysSpawn" "OverrideRootScale" null (`self.Overlapping`) Type null))
        (`self.K2_AttachToComponent` _returnvalue (`self.ProceduralMesh`) "None" "KeepRelative" "KeepRelative" "KeepRelative" true)
        (else
          (bind _returnvalue_2 (`|SpawnActorFromClass` "/Game/Blueprints/Fill.Fill_C" (`KismetMathLibrary.MakeTransform` (0.0 0.0 0.0) (struct) (1.0 1.0 1.0)) "AlwaysSpawn" "OverrideRootScale" null (`self.Overlapping`) Type null))
          (`self.K2_AttachToComponent` _returnvalue_2 (`self.ProceduralMesh1`) "None" "KeepRelative" "KeepRelative" "KeepRelative" true))))))

(fn `GetPlayerOrientation`
  (params (Pawn :type "/Game/Blueprints/VR_Pawn Object Reference (by ref)") (DoorCollision :type "BoxComponent Object Reference (by ref)"))
  (returns (Direction :type Boolean) (Location :type Boolean))
  (bind (_returnvalue_x _returnvalue_y) (`KismetMathLibrary.BreakVector` (`SceneComponent.K2_GetComponentLocation` DoorCollision)))
  (bind (_returnvalue_x_2 _returnvalue_y_2) (`KismetMathLibrary.BreakVector` (`SceneComponent.K2_GetComponentLocation` DoorCollision)))
  (bind (_returnvalue_x_3 _returnvalue_y_3) (`KismetMathLibrary.BreakVector` (`SceneComponent.K2_GetComponentLocation` (`self.B`))))
  (bind _returnvalue (`SceneComponent.K2_GetComponentLocation` (`/Game/Blueprints/VR_Pawn.SphereCollision` Pawn)))
  (bind _returnvalue_2 (- (`KismetMathLibrary.MakeVector` _returnvalue_x_3 _returnvalue_y_3) (`KismetMathLibrary.MakeVector` _returnvalue_x_2 _returnvalue_y_2)))
  (bind _returnvalue_3 (* _returnvalue_2 100.0))
  (return (> (`KismetMathLibrary.Dot_VectorVector` _returnvalue_2 (`/Game/Blueprints/VR_Pawn.DirectionOfTravel` Pawn)) 0.0) (< (`KismetMathLibrary.VSizeXYSquared` (- (- (`KismetMathLibrary.MakeVector` _returnvalue_x _returnvalue_y) _returnvalue_3) _returnvalue)) (`KismetMathLibrary.VSizeXYSquared` (- (+ (`KismetMathLibrary.MakeVector` _returnvalue_x _returnvalue_y) _returnvalue_3) _returnvalue)))))

(fn `Marker`
  (params (Marker :type "BoxComponent Object Reference"))
  (for _array_element (`PrimitiveComponent.GetOverlappingComponents` Marker)
    (bind _returnvalue (`ActorComponent.GetOwner` _array_element))
    (if (!= _returnvalue self)
      (bind _asdoor (cast `/Game/Blueprints/Door` _returnvalue))
      (if (`KismetStringLibrary.Contains` (`KismetSystemLibrary.GetDisplayName` _array_element) "Overlapping")
        (`self.Attach` _asdoor (`self.Overlapping`))
        (`KismetArrayLibrary.Array_Add` (`self.AttachedActor`) _asdoor)))))

(fn `SceneControl`
  (params (DoorCollision :type "BoxComponent Object Reference (by ref)"))
  (bind _returnvalue (`GameplayStatics.GetPlayerController` 0))
  (if (and (`PrimitiveComponent.IsOverlappingComponent` (`self.A`) DoorCollision) (`KismetStringLibrary.NotEqual_StrStr` (`self.CurrentScene`) "A"))
    (set `self.CurrentScene` "A")
    (message `/Game/Blueprints/StoryInterface.NextScene` _returnvalue)
    (elif (and (`PrimitiveComponent.IsOverlappingComponent` (`self.B`) DoorCollision) (`KismetStringLibrary.NotEqual_StrStr` (`self.CurrentScene`) "B"))
      (set `self.CurrentScene` "B")
      (message `/Game/Blueprints/StoryInterface.PreviousScene` _returnvalue))))

(fn `SetPivotAtMidpoint`
  (params (InputVector :type "Array of Vector Structure (by ref)"))
  (returns (OutputVector :type "Array of Vector Structure"))
  (locals (x_min :type "Float (double-precision)") (x_max :type "Float (double-precision)"))
  (for _array_element InputVector
    (if (< (.x _array_element) (`local.x_min`))
      (bind _output_get (set `local.x_min` (.x _array_element))))
    (if (> (.x _array_element) (`local.x_max`))
      (bind _output_get_2 (set `local.x_max` (.x _array_element))))
    (for (_array_element_2 _array_index) InputVector
      (`KismetArrayLibrary.Array_Set` InputVector _array_index (`KismetMathLibrary.MakeVector` (- (.x _array_element_2) (`KismetMathLibrary.Abs` (/ (- _output_get_2 _output_get) 2.0)))))
      (return InputVector))))

(fn `UserConstructionScript`
  (bind _doorcollision2 (`self.DoorCollision2`))
  (bind _c (`self.C`))
  (bind _proceduralmesh (`self.ProceduralMesh`))
  (bind _doorwidth (`self.DoorWidth`))
  (bind _d (`self.D`))
  (bind _a (`self.A`))
  (bind _overlapping (`self.Overlapping`))
  (bind _height (`self.Height`))
  (bind _b (`self.B`))
  (bind _proceduralmesh1 (`self.ProceduralMesh1`))
  (bind _doorcollision1 (`self.DoorCollision1`))
  (bind _returnvalue (/ (`self.Width`) 2.0))
  (bind _returnvalue_2 (/ (`self.Height`) 2.0))
  (bind _returnvalue_3 (/ (`self.Width`) 2.0))
  (bind _returnvalue_4 (* _height -1.0))
  (bind _returnvalue_5 (- _returnvalue 30.0))
  (`|ExecutionSequence`
    (:`then_0`
      ;[0 0 0] SetUp DoorPosition
      (for _array_element (`self.DoorPos%`)
        (if (> _array_element 0.5)
          (bind _returnvalue_6 (* (`self.Width`) _array_element))
          (`KismetArrayLibrary.Array_Add` (`self.DoorRightPts`) _returnvalue_6)
          (`KismetArrayLibrary.Array_Add` (`self.DoorLeftPts`) (- _returnvalue_6 _doorwidth))
          (elif (== _array_element 0.5)
            (bind _returnvalue_7 (- _returnvalue_6 (/ _doorwidth 2.0)))
            (`KismetArrayLibrary.Array_Add` (`self.DoorLeftPts`) _returnvalue_7)
            (`KismetArrayLibrary.Array_Add` (`self.DoorRightPts`) (+ _doorwidth _returnvalue_7))
            (else
              (`KismetArrayLibrary.Array_Add` (`self.DoorLeftPts`) _returnvalue_6)
              (`KismetArrayLibrary.Array_Add` (`self.DoorRightPts`) (+ _returnvalue_6 _doorwidth)))))))
    (:`then_1`
      ;[0 0 0] Make ProceduralMesh
      (`|ExecutionSequence`
        (:`then_0`
          (`self.CalculateMeshPts` (`self.DoorNum`))
          (`ProceduralMeshComponent.CreateMeshSection_LinearColor` :`self` _proceduralmesh :`Vertices` (`self.vertices`) :`Triangles` (`self.triangles`) :`UV0` (`self.UV`) :`bCreateCollision` true)
          (`PrimitiveComponent.SetMaterial` _proceduralmesh 0 (`self.Material`)))
        (:`then_1`
          (`self.CalculateMeshPts` (`self.DoorNum1`))
          (`ProceduralMeshComponent.CreateMeshSection_LinearColor` :`self` _proceduralmesh1 :`Vertices` (`self.vertices`) :`Triangles` (`self.triangles`) :`UV0` (`self.UV`) :`bCreateCollision` true)
          (`PrimitiveComponent.SetMaterial` _proceduralmesh1 0 (`self.Material1`)))))
    (:`then_2`
      ;[0 0 0] DoorCollision
      (if (`self.NoDoor`)
        (`ActorComponent.K2_DestroyComponent` _doorcollision1)
        (`ActorComponent.K2_DestroyComponent` _doorcollision2 :!label _label)
        (else
          (`self.CalculateDoorCollision` _doorcollision1)
          (if (> (`KismetArrayLibrary.Array_Length` (`self.DoorPos%`)) 1)
            (`self.CalculateDoorCollision` _doorcollision2 1)
            (else
              (goto _label))))))
    (:`then_3`
      ;[0 0 0] overlapping Collision
      (`BoxComponent.SetBoxExtent` _overlapping (`KismetMathLibrary.MakeVector` _returnvalue_3 _returnvalue_2 2.5) true)
      (`SceneComponent.K2_SetRelativeLocation` _overlapping (`KismetMathLibrary.MakeVector` _returnvalue_3 _returnvalue_2) false false)
      (`SceneComponent.K2_AttachToComponent` (`self.Overlapping`) (`self.ProceduralMesh`) "None" "KeepRelative" "KeepRelative" "KeepRelative" true))
    (:`then_4`
      ;[0 0 0] Markers: A B C D
      (`|ExecutionSequence`
        (:`then_0`
          (`SceneComponent.K2_SetRelativeLocation` _b (`KismetMathLibrary.MakeVector` _returnvalue _height) false false)
          (`SceneComponent.K2_SetRelativeLocation` _a (`KismetMathLibrary.MakeVector` _returnvalue _returnvalue_4) false false)
          (`SceneComponent.K2_SetRelativeLocation` _c (`KismetMathLibrary.MakeVector` _returnvalue 0.0 _height) false false)
          (`SceneComponent.K2_SetRelativeLocation` _d (`KismetMathLibrary.MakeVector` _returnvalue 0.0 _returnvalue_4) false false))
        (:`then_1`
          (`BoxComponent.SetBoxExtent` _b (`KismetMathLibrary.MakeVector` _returnvalue_5 3.0 3.0) true)
          (`BoxComponent.SetBoxExtent` _a (`KismetMathLibrary.MakeVector` _returnvalue_5 3.0 3.0) true)
          (`BoxComponent.SetBoxExtent` _c (`KismetMathLibrary.MakeVector` _returnvalue_5 3.0 3.0) true)
          (`BoxComponent.SetBoxExtent` _d (`KismetMathLibrary.MakeVector` _returnvalue_5 3.0 3.0) true))))))