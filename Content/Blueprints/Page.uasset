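; Page is a two-sided procedural panel with an optional door cutout that swings about its base edge, spawning themed Fill content on each face.
; Construction builds both meshes, door frame, trigger and edge markers.
; VR pawn overlaps at the door pick one of two rotation timelines from travel direction and side.
; Neighboring Pages found through the markers, and overlapping pickup actors, get attachment calls around rotations.
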(event `self.ReceiveTick`
  (params (DeltaSeconds :type "Float (single-precision)")))

(event `self.ReceiveBeginPlay`
  ;[0 0 0] BeginPlay
  (`self.AttachActors`)
  ;[0 0 0] Spawn Fill
  (`self.SpawnContent` (`self.ProceduralMesh`) (`self.Page`))
  (`self.SpawnContent` (`self.ProceduralMesh1`) (`self.Page1`) true))

(event `Attach`
  (params (Parent :type "SceneComponent Object Reference"))
  ;[0 0 0] AttachDoor
  (`self.K2_AttachToComponent` Parent "None" "KeepWorld" "KeepWorld" "KeepWorld"))

(event `Detach`
  ;[0 0 0] AttachDoor
  (`self.K2_DetachFromActor` "KeepWorld" "KeepWorld" "KeepWorld"))

(event `/Game/Blueprints/DoorInterface.Open`
  ;[0 0 0] Determine Opening Direction of Door
  (`self.AttachActors`)
  ;[0 0 0] Open Door
  (`self.AttachDoor`)
  (bind (_direction _90) (`Timeline|Timeline_0` :!label _label)
    (:`Update`
      (`SceneComponent.K2_SetRelativeRotation` (`self.ProceduralMesh`) (`KismetMathLibrary.MakeRotator` (* _90 (`self.Angle`))) false false))
    (:`Finished`
      (`self.DetachDoor` :!label _label_2))))

(event `/Game/Blueprints/DoorInterface.Open2`
  ;[0 0 0] Determine Opening Direction of Door
  (`self.AttachActors`)
  ;[0 0 0] Open Door
  (`self.AttachDoor`)
  (bind (_direction _90) (`Timeline|90_180` :!label _label_3)
    (:`Update`
      (`SceneComponent.K2_SetRelativeRotation` (`self.ProceduralMesh`) (`KismetMathLibrary.MakeRotator` (* _90 (`self.Angle`))) false false))
    (:`Finished`
      (goto _label_2))))

(event `self.DoorCollision1.OnComponentBeginOverlap`
  (params (OverlappedComponent :type "PrimitiveComponent Object Reference") (OtherActor :type "Actor Object Reference") (OtherComp :type "PrimitiveComponent Object Reference") (OtherBodyIndex :type Integer) (bFromSweep :type Boolean) (SweepResult :type "HitResult Structure (by ref)"))
  (bind _returnvalue_roll (`KismetMathLibrary.BreakRotator` (`SceneComponent.K2_GetComponentRotation` (`self.ProceduralMesh`))))
  (bind _returnvalue (< (`KismetMathLibrary.Abs` _returnvalue_roll) 90.0))
  ;[0 0 0] Determine Opening Direction of Door
  (bind _asvr_pawn (cast `/Game/Blueprints/VR_Pawn` OtherActor))
  (`|ExecutionSequence`
    (:`then_0`
      (`self.AttachActors`))
    (:`then_1`
      (`self.AttachDoor`))
    (:`then_2`
      (bind (_direction _location) (`self.GetPlayerOrientation` _asvr_pawn))
      (if (and _direction _location _returnvalue)
        (goto _label)
        (elif (and (not _direction) (not _location) (not _returnvalue))
          (goto _label_3 :!via `Reverse`))))))

(event `self.DoorCollision1.OnComponentEndOverlap`
  (params (OverlappedComponent :type "PrimitiveComponent Object Reference") (OtherActor :type "Actor Object Reference") (OtherComp :type "PrimitiveComponent Object Reference") (OtherBodyIndex :type Integer))
  ;[0 0 0] Determine Opening Direction of Door
  (bind _asvr_pawn (cast `/Game/Blueprints/VR_Pawn` OtherActor))
  (`|ExecutionSequence`
    (:`then_0`
      (`self.AttachActors`))
    (:`then_1`
      (bind (_direction _location) (`self.GetPlayerOrientation` _asvr_pawn))
      (if (and (not _direction) _location)
        (set `self.Clockwise` true)
        (goto _label :!via `Reverse`)
        (elif (and _direction (not _location))
          (set `self.Clockwise` false)
          (goto _label_3))))
    (:`then_2`
      (`self.AttachDoor`))))

(event `/Game/Blueprints/DoorInterface.Close`
  ;[0 0 0] Determine Opening Direction of Door
  (`self.AttachActors`)
  ;[0 0 0] Open Door
  (`self.AttachDoor`)
  (goto _label_3 :!via `Reverse`))

(event `/Game/Blueprints/DoorInterface.Close1`
  ;[0 0 0] Determine Opening Direction of Door
  (`self.AttachDoor`)
  ;[0 0 0] Open Door
  (`self.AttachActors`)
  (goto _label_3))

(fn `AttachActors`
  (for _array_element (`PrimitiveComponent.GetOverlappingActors` (`self.Overlapping`) "/Script/Engine.Actor")
    (if (`KismetSystemLibrary.DoesImplementInterface` _array_element "/Game/Blueprints/PickupActorInterface.PickupActorInterface_C")
      (message `/Game/Blueprints/PickupActorInterface.Pickup` _array_element (`self.ProceduralMesh`)))))

(fn `AttachDoor`
  (locals (OriginalPosition :type "Vector Structure" :default (0.0 0.0 0.0)))
  (bind _d (`self.D`))
  (bind _b (`self.B`))
  (bind _a (`self.A`))
  ;[1 1 1] Find Overlapping Door on Marker
  (for _array_element (`PrimitiveComponent.GetOverlappingComponents` (`self.Overlapping`))
    (if (and (!= _array_element (`self.DoorCollision1`)) (!= _array_element (`self.ProceduralMesh`)) (== (`ActorComponent.GetOwner` _array_element) self))
      (bind _output_get (set `self.CurrentMarker` (`.RightS` (`KismetStringLibrary.Split` (`KismetSystemLibrary.GetDisplayName` _array_element) "."))))
      ;[1 1 1] Depending on Marker, attach 'x' Door
      (switch `string` _output_get
        (:`A`
          (`self.Marker` (`self.A`))
          (bind _output_get_2 (set `local.OriginalPosition` (`SceneComponent.RelativeLocation` _d) :!label _label))
          (`SceneComponent.K2_SetRelativeLocation` _d (`KismetMathLibrary.MakeVector` (/ (`self.Width`) 2.0) 0.0 -50.0) false false)
          (`self.Marker` _d)
          (`SceneComponent.K2_SetRelativeLocation` _d _output_get_2 false false))
        (:`B`
          (`self.Marker` (`self.B`))
          (goto _label))
        (:`C`
          (`self.Marker` (`self.C`))
          (if (`self.Clockwise`)
            (bind _output_get_3 (set `local.OriginalPosition` (`SceneComponent.RelativeLocation` _b)))
            (`SceneComponent.K2_SetRelativeLocation` _b (`KismetMathLibrary.MakeVector` (/ (`self.Width`) 2.0) 50.0) false false)
            (`self.Marker` _b)
            (`SceneComponent.K2_SetRelativeLocation` _b _output_get_3 false false)
            (else
              (bind _output_get_4 (set `local.OriginalPosition` (`SceneComponent.RelativeLocation` _a)))
              (`SceneComponent.K2_SetRelativeLocation` _a (`KismetMathLibrary.MakeVector` (/ (`self.Width`) 2.0) -50.0) false false)
              (`self.Marker` _a)
              (`SceneComponent.K2_SetRelativeLocation` _a _output_get_4 false false))))
        (:`D`
          (`self.Marker` (`self.D`)))))))

(fn `DetachDoor`
  (bind _attachedactor (`self.AttachedActor`))
  (for _array_element _attachedactor
    (bind _aspage (cast `/Game/Blueprints/Page` _array_element))
    (`self.Detach` _aspage))
  (`KismetArrayLibrary.Array_Clear` _attachedactor))

(fn `GetPlayerOrientation`
  (params (Pawn :type "/Game/Blueprints/VR_Pawn Object Reference"))
  (returns (Direction :type Boolean) (Location :type Boolean))
  (bind (_returnvalue_x _returnvalue_y) (`KismetMathLibrary.BreakVector` (`SceneComponent.K2_GetComponentLocation` (`self.DoorCollision1`))))
  (bind (_returnvalue_x_2 _returnvalue_y_2) (`KismetMathLibrary.BreakVector` (`SceneComponent.K2_GetComponentLocation` (`self.B`))))
  (bind (_returnvalue_x_3 _returnvalue_y_3) (`KismetMathLibrary.BreakVector` (`SceneComponent.K2_GetComponentLocation` (`self.DoorCollision1`))))
  (bind _returnvalue (`SceneComponent.K2_GetComponentLocation` (`/Game/Blueprints/VR_Pawn.SphereCollision` Pawn)))
  (bind _returnvalue_2 (- (`KismetMathLibrary.MakeVector` _returnvalue_x_2 _returnvalue_y_2) (`KismetMathLibrary.MakeVector` _returnvalue_x_3 _returnvalue_y_3)))
  (bind _returnvalue_3 (* _returnvalue_2 100.0))
  (return (> (`KismetMathLibrary.Dot_VectorVector` _returnvalue_2 (`/Game/Blueprints/VR_Pawn.DirectionOfTravel` Pawn)) 0.0) (< (`KismetMathLibrary.VSizeXYSquared` (- (- (`KismetMathLibrary.MakeVector` _returnvalue_x _returnvalue_y) _returnvalue_3) _returnvalue)) (`KismetMathLibrary.VSizeXYSquared` (- (+ (`KismetMathLibrary.MakeVector` _returnvalue_x _returnvalue_y) _returnvalue_3) _returnvalue)))))

(fn `Marker`
  (params (Marker :type "BoxComponent Object Reference"))
  (for _array_element (`PrimitiveComponent.GetOverlappingComponents` Marker)
    (bind _returnvalue (`ActorComponent.GetOwner` _array_element))
    (if (!= _returnvalue self)
      (bind _aspage (cast `/Game/Blueprints/Page` _returnvalue))
      (if (`KismetStringLibrary.Contains` (`KismetSystemLibrary.GetDisplayName` _array_element) "Overlapping")
        (`self.Attach` (`self.Overlapping`))
        (`KismetArrayLibrary.Array_Add` (`self.AttachedActor`) _aspage)))))

(fn `SetPivotAtMidpoint`
  (params (InputVector :type "Array of Vector Structure (by ref)"))
  (returns (OutputVector :type "Array of Vector Structure"))
  (locals (x_min :type "Float (double-precision)") (x_max :type "Float (double-precision)"))
  (for _array_element InputVector
    (if (< (.x _array_element) (`local.x_min`))
      (bind _output_get (set `local.x_min` (.x _array_element))))
    (if (> (.x _array_element) (`local.x_max`))
      (bind _output_get_2 (set `local.x_max` (.x _array_element))))
    (for (_array_element_2 _array_index) InputVector
      (`KismetArrayLibrary.Array_Set` InputVector _array_index (`KismetMathLibrary.MakeVector` (- (.x _array_element_2) (`KismetMathLibrary.Abs` (/ (- _output_get_2 _output_get) 2.0)))))
      (return InputVector))))

(fn `SpawnContent`
  (params (ProceduralMesh :type "ProceduralMeshComponent Object Reference") (Type :type "/Game/Blueprints/PageEnum Enum" :default "NewEnumerator0") (OtherSide :type Boolean))
  (locals (side :type "Float (double-precision)"))
  (`|ExecutionSequence`
    (:`then_0`
      (switch `/Game/Blueprints/PageEnum` Type
        (:`NewEnumerator0`
          (`PrimitiveComponent.SetMaterial` ProceduralMesh 0 "/Game/Floor/M_Ground_Grass.M_Ground_Grass"))
        (:`NewEnumerator1`
          (`PrimitiveComponent.SetMaterial` ProceduralMesh 0 "/Game/Imports/Seaside_Town/Materials/Tilables/MI_Floors_Stone_Inst4.MI_Floors_Stone_Inst4"))
        (:`NewEnumerator2`
          (`PrimitiveComponent.SetMaterial` ProceduralMesh 0 "/Game/Floor/M_URockB.M_URockB"))
        (:`NewEnumerator3`
          (`PrimitiveComponent.SetMaterial` ProceduralMesh 0 "/Game/Imports/FreeFurniturePack/Materials/M_Chrome.M_Chrome"))
        (:`NewEnumerator4`
          (`PrimitiveComponent.SetMaterial` ProceduralMesh 0 "/Game/Floor/M_Basic_Wall.M_Basic_Wall"))
        (:`NewEnumerator5`
          (`PrimitiveComponent.SetMaterial` ProceduralMesh 0 "/Game/Floor/M_Wood_Floor_Walnut_Polished.M_Wood_Floor_Walnut_Polished"))))
    (:`then_1`
      (if OtherSide
        (set `local.side` -1.0)
        (else
          (set `local.side` 1.0)))
      (bind _returnvalue (`|SpawnActorFromClass` "/Game/Blueprints/Fill.Fill_C" (`KismetMathLibrary.MakeTransform` (0.0 0.0 0.0) (struct) (`KismetMathLibrary.MakeVector` 1.0 1.0 (`local.side`))) "AlwaysSpawn" "OverrideRootScale" null (`self.Overlapping`) Type (`self.PublicDoorLeft`) (`self.DoorHeight`) (`self.DoorWidth`) null))
      (`self.K2_AttachToComponent` _returnvalue ProceduralMesh "None" "KeepRelative" "KeepRelative" "KeepRelative" true))))

(fn `UserConstructionScript`
  (locals (DoorLeftPt :type "Float (double-precision)" :default 150.0) (DoorRightPt :type "Float (double-precision)" :default 250.0) (DoorFrameWidth :type "Float (double-precision)" :default 2.5))
  (bind _array (`|MakeArray` (0.0 0.0) (0.0 1.0) (0.5 1.0) (1.0 1.0) (1.0 0.0) (0.6 0.0) (0.6 0.8) (0.3 0.8) (0.3 0.0) :!type "Vector2D Structure"))
  (bind _d (`self.D`))
  (bind _doorrightpt (`local.DoorRightPt`))
  (bind _doorcollision1 (`self.DoorCollision1`))
  (bind _doorleftpt (`local.DoorLeftPt`))
  (bind _proceduralmesh (`self.ProceduralMesh`))
  (bind _proceduralmesh_2 (`self.ProceduralMesh`))
  (bind _doorwidth (`self.DoorWidth`))
  (bind _doorleftpt_2 (`local.DoorLeftPt`))
  (bind _doorframewidth (`local.DoorFrameWidth`))
  (bind _a (`self.A`))
  (bind _overlapping (`self.Overlapping`))
  (bind _doorheight (`self.DoorHeight`))
  (bind _doorposition_ (`self.DoorPosition%`))
  (bind _height (`self.Height`))
  (bind _b (`self.B`))
  (bind _doorframe (`self.DoorFrame`))
  (bind _c (`self.C`))
  (bind _doorheight_2 (`self.DoorHeight`))
  (bind _doorrightpt_2 (`local.DoorRightPt`))
  (bind _doorframewidth_2 (`local.DoorFrameWidth`))
  (bind _height_2 (`self.Height`))
  (bind _proceduralmesh1 (`self.ProceduralMesh1`))
  (bind _width (`self.Width`))
  (bind _returnvalue (/ (`self.DoorHeight`) 2.0))
  (bind _returnvalue_2 (/ (`self.Width`) 2.0))
  (bind _returnvalue_3 (/ (`self.Height`) 2.0))
  (bind _returnvalue_4 (/ (`self.Width`) 2.0))
  (bind _returnvalue_5 (* -1 _doorframewidth_2))
  (bind _returnvalue_6 (* _height -1.0))
  (bind _returnvalue_7 (* (`self.Width`) _doorposition_))
  (bind _returnvalue_8 (- _returnvalue_2 30.0))
  (bind _array_2 (`|MakeArray` (0.0 0.0 0.0) (`KismetMathLibrary.MakeVector` 0.0 _height_2) (`KismetMathLibrary.MakeVector` (/ _width 2.0) _height_2) (`KismetMathLibrary.MakeVector` _width _height_2) (`KismetMathLibrary.MakeVector` _width) (`KismetMathLibrary.MakeVector` _doorrightpt) (`KismetMathLibrary.MakeVector` _doorrightpt _doorheight) (`KismetMathLibrary.MakeVector` _doorleftpt _doorheight) (`KismetMathLibrary.MakeVector` _doorleftpt) :!type "Vector Structure"))
  (`|ExecutionSequence`
    (:`then_0`
      ;[0 0 0] SetUp DoorPosition
      (if (> _doorposition_ 0.5)
        (bind _output_get (set `local.DoorRightPt` _returnvalue_7)) ; Door located right
        (set `local.DoorLeftPt` (- _output_get _doorwidth))
        (elif (== (`self.DoorPosition%`) 0.5)
          (bind _output_get_2 (set `local.DoorLeftPt` (- _returnvalue_7 (/ _doorwidth 2.0)))) ; Door  located at midpt?
          (set `local.DoorRightPt` (+ _doorwidth _output_get_2))
          (else
            (bind _output_get_3 (set `local.DoorLeftPt` _returnvalue_7)) ; Door located towards the left
            (set `local.DoorRightPt` (+ _output_get_3 _doorwidth))))))
    (:`then_1`
      ;[0 0 0] Make ProceduralMesh
      (set `self.PublicDoorLeft` (`local.DoorLeftPt`))
      (`ProceduralMeshComponent.CreateMeshSection_LinearColor` :`self` _proceduralmesh_2 :`Vertices` _array_2 :`Triangles` (`|MakeArray` 0 7 8 0 1 7 1 2 7 7 2 6 6 2 3 3 4 6 4 5 6) :`UV0` _array :`bCreateCollision` true)
      (`PrimitiveComponent.SetMaterial` _proceduralmesh_2 0 (`self.Material`))
      ;[0 0 0] Make ProceduralMesh
      (`|ExecutionSequence`
        (:`then_0`
          (set `self.vertices` _array_2)
          (for (_ _array_index) _array
            (`KismetArrayLibrary.Array_Add` (`self.UV`) (`|GetArrayItem` _array (- (`KismetArrayLibrary.Array_LastIndex` _array) _array_index)))))
        (:`then_1`
          (set `self.triangles` (`|MakeArray` 0 8 7 0 7 1 1 7 2 7 6 2 6 3 2 3 6 4 4 6 5))
          (`ProceduralMeshComponent.CreateMeshSection_LinearColor` :`self` _proceduralmesh1 :`Vertices` (`self.vertices`) :`Triangles` (`self.triangles`) :`UV0` (`self.UV`) :`bCreateCollision` true)
          (`PrimitiveComponent.SetMaterial` _proceduralmesh1 0 (`self.Material1`)))))
    (:`then_2`
      ;[0 0 0] DoorCollision
      (if (`self.NoDoor`)
        (`ActorComponent.K2_DestroyComponent` _doorcollision1)
        (else
          (`BoxComponent.SetBoxExtent` _doorcollision1 (`KismetMathLibrary.MakeVector` (/ (`self.DoorWidth`) 5.0) 2.5 _returnvalue) true)
          (`SceneComponent.K2_SetRelativeLocation` _doorcollision1 (`KismetMathLibrary.MakeVector` (/ (+ (`local.DoorLeftPt`) (`local.DoorRightPt`)) 2.0) -2.5 _returnvalue) false false))))
    (:`then_3`
      ;[0 0 0] overlapping Collision
      (`BoxComponent.SetBoxExtent` _overlapping (`KismetMathLibrary.MakeVector` _returnvalue_4 _returnvalue_3 2.5) true)
      (`SceneComponent.K2_SetRelativeLocation` _overlapping (`KismetMathLibrary.MakeVector` _returnvalue_4 _returnvalue_3) false false)
      (`SceneComponent.K2_AttachToComponent` (`self.Overlapping`) _proceduralmesh "None" "KeepRelative" "KeepRelative" "KeepRelative" true)
      (`SceneComponent.K2_AttachToComponent` (`self.ProceduralMesh1`) _proceduralmesh "None" "KeepRelative" "KeepRelative" "KeepRelative" true))
    (:`then_4`
      ;[0 0 0] Markers: A B C D
      (`|ExecutionSequence`
        (:`then_0`
          (`SceneComponent.K2_SetRelativeLocation` _b (`KismetMathLibrary.MakeVector` _returnvalue_2 _height) false false)
          (`SceneComponent.K2_SetRelativeLocation` _a (`KismetMathLibrary.MakeVector` _returnvalue_2 _returnvalue_6) false false)
          (`SceneComponent.K2_SetRelativeLocation` _c (`KismetMathLibrary.MakeVector` _returnvalue_2 0.0 _height) false false)
          (`SceneComponent.K2_SetRelativeLocation` _d (`KismetMathLibrary.MakeVector` _returnvalue_2 0.0 _returnvalue_6) false false))
        (:`then_1`
          (`BoxComponent.SetBoxExtent` _b (`KismetMathLibrary.MakeVector` _returnvalue_8 3.0 3.0) true)
          (`BoxComponent.SetBoxExtent` _a (`KismetMathLibrary.MakeVector` _returnvalue_8 3.0 3.0) true)
          (`BoxComponent.SetBoxExtent` _c (`KismetMathLibrary.MakeVector` _returnvalue_8 3.0 3.0) true)
          (`BoxComponent.SetBoxExtent` _d (`KismetMathLibrary.MakeVector` _returnvalue_8 3.0 3.0) true))))
    (:`then_5`
      ;[0 0 0] Make Door Frame
      (if (`self.NoDoor`)
        (`ActorComponent.K2_DestroyComponent` (`self.DoorFrame`))
        (else
          (`ProceduralMeshComponent.CreateMeshSection_LinearColor` :`self` _doorframe :`Vertices` (`|MakeArray` (`KismetMathLibrary.MakeVector` _doorleftpt_2 _doorframewidth_2) (`KismetMathLibrary.MakeVector` _doorleftpt_2 _returnvalue_5) (`KismetMathLibrary.MakeVector` _doorleftpt_2 _returnvalue_5 _doorheight_2) (`KismetMathLibrary.MakeVector` _doorrightpt_2 _returnvalue_5 _doorheight_2) (`KismetMathLibrary.MakeVector` _doorrightpt_2 _returnvalue_5) (`KismetMathLibrary.MakeVector` _doorrightpt_2 _doorframewidth) (`KismetMathLibrary.MakeVector` _doorrightpt_2 _doorframewidth _doorheight_2) (`KismetMathLibrary.MakeVector` _doorleftpt_2 _doorframewidth _doorheight_2) :!type "Vector Structure") :`Triangles` (`|MakeArray` 0 1 2 0 2 7 2 3 6 2 6 7 3 4 5 3 5 6) :`UV0` (`|MakeArray` (0.0 0.0) (0.2 0.0) (0.2 1.0) (0.2 0.0) (0.2 1.0) (0.0 1.0) (0.0 0.0) (0.0 1.0) :!type "Vector2D Structure") :`bCreateCollision` true)
          (`SceneComponent.K2_AttachToComponent` _doorframe null "None" "KeepRelative" "KeepRelative" "KeepRelative" true)
          (`PrimitiveComponent.SetMaterial` _doorframe 0 "/Game/VirtualReality/Materials/M_ArcEndpoint.M_ArcEndpoint"))))))