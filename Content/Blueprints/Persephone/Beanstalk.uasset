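; Beanstalk Blueprint in the Persephone folder, apparently an unfinished growth effect for a beanstalk built from numbered meshes.
; BeginPlay starts a fast looping timer on a Tick1 event, which has no logic attached.
; A disconnected switch on Count would pass each mesh to IncreaseSize, whose body is empty, and a stray node would zero the last mesh's scale.
; As it stands, nothing visibly grows.
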(event `self.ReceiveBeginPlay`
  (`KismetSystemLibrary.K2_SetTimerDelegate` (delegate `Tick1`) 0.05 true))

(event `Tick1`)

(fn `IncreaseSize`
  (params (Mesh :type "StaticMeshComponent Object Reference (by ref)")))

(fn `UserConstructionScript`)