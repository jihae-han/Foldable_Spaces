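; HoriAnchor is an anchor actor that builds a scene from six Hori actors configured by SceneMap entries.
; Its construction script offsets markers A–D and sizes four door overlap boxes, disabling overlaps on two.
; SetupScene calls Spawn, which sets roll by marker and mirrors even-indexed pieces with negative Z scale, taking their door data from the preceding entry.
; SetupScene also repositions the first door box, while the overlap handlers remain stubs.
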(event `self.DoorCollision1.OnComponentBeginOverlap`
  (params (OverlappedComponent :type "PrimitiveComponent Object Reference") (OtherActor :type "Actor Object Reference") (OtherComp :type "PrimitiveComponent Object Reference") (OtherBodyIndex :type Integer) (bFromSweep :type Boolean) (SweepResult :type "HitResult Structure (by ref)"))
  ;[1 1 1] Door1
  (cast `/Game/Blueprints/Test_Pawn` OtherActor))

(event `self.DoorCollision1.OnComponentEndOverlap`
  (params (OverlappedComponent :type "PrimitiveComponent Object Reference") (OtherActor :type "Actor Object Reference") (OtherComp :type "PrimitiveComponent Object Reference") (OtherBodyIndex :type Integer))
  ;[1 1 1] Door1
)

(event `self.DoorCollision3.OnComponentBeginOverlap`
  (params (OverlappedComponent :type "PrimitiveComponent Object Reference") (OtherActor :type "Actor Object Reference") (OtherComp :type "PrimitiveComponent Object Reference") (OtherBodyIndex :type Integer) (bFromSweep :type Boolean) (SweepResult :type "HitResult Structure (by ref)"))
  ;[1 1 1] Door1
)

(event `self.DoorCollision3.OnComponentEndOverlap`
  (params (OverlappedComponent :type "PrimitiveComponent Object Reference") (OtherActor :type "Actor Object Reference") (OtherComp :type "PrimitiveComponent Object Reference") (OtherBodyIndex :type Integer))
  ;[1 1 1] Door1
)

(event `self.DoorCollision2.OnComponentBeginOverlap`
  (params (OverlappedComponent :type "PrimitiveComponent Object Reference") (OtherActor :type "Actor Object Reference") (OtherComp :type "PrimitiveComponent Object Reference") (OtherBodyIndex :type Integer) (bFromSweep :type Boolean) (SweepResult :type "HitResult Structure (by ref)"))
  ;[0 0 0] Door2
)

(event `self.DoorCollision2.OnComponentEndOverlap`
  (params (OverlappedComponent :type "PrimitiveComponent Object Reference") (OtherActor :type "Actor Object Reference") (OtherComp :type "PrimitiveComponent Object Reference") (OtherBodyIndex :type Integer))
  ;[0 0 0] Door2
)

(event `self.DoorCollision4.OnComponentBeginOverlap`
  (params (OverlappedComponent :type "PrimitiveComponent Object Reference") (OtherActor :type "Actor Object Reference") (OtherComp :type "PrimitiveComponent Object Reference") (OtherBodyIndex :type Integer) (bFromSweep :type Boolean) (SweepResult :type "HitResult Structure (by ref)"))
  ;[0 0 0] Door2
)

(event `self.DoorCollision4.OnComponentEndOverlap`
  (params (OverlappedComponent :type "PrimitiveComponent Object Reference") (OtherActor :type "Actor Object Reference") (OtherComp :type "PrimitiveComponent Object Reference") (OtherBodyIndex :type Integer))
  ;[0 0 0] Door2
)

(fn `SetupScene`
  (`|ExecutionSequence`
    (:`then_0`
      (`self.Spawn` 0 "A")
      (`self.Spawn` 1 "B")
      (`self.Spawn` 2 "B")
      (`self.Spawn` 3 "D")
      (`self.Spawn` 4 "D")
      (`self.Spawn` 5 "A"))
    (:`then_1`
      (`SceneComponent.K2_SetRelativeLocation` (`self.DoorCollision1`) (`KismetMathLibrary.MakeVector` (`.DoorPos_19_C2E507344DDC2E97812767A97C245227` (break `/Game/Blueprints/SceneSaver` (`BlueprintMapLibrary.Map_Find` (`self.SceneMap`) 1))) -5.0 (/ (`self.DoorHeight`) 2.0)) false false)
      (`KismetSystemLibrary.PrintString` (`KismetStringLibrary.Conv_DoubleToString` 0.0)))))

(fn `Spawn`
  (params (Scene :type Integer) (Marker :type String))
  (locals (`tempDoor?` :type Boolean) (RotationX :type "Float (double-precision)"))
  (bind (_value _returnvalue) (`BlueprintMapLibrary.Map_Find` (`self.SceneMap`) Scene))
  (bind (_value_2 _returnvalue_2) (`BlueprintMapLibrary.Map_Find` (`self.SceneMap`) (- Scene 1)))
  (`|ExecutionSequence`
    (:`then_0`
      (switch `string` Marker
        (:`A`
          (set `local.RotationX` 180.0))
        (:`B`
          (set `local.RotationX` 0.0))
        (:`D`
          (set `local.RotationX` 90.0))))
    (:`then_1`
      (if _returnvalue
        (if (> (mod Scene 2) 0)
          (`|SpawnActorFromClass` "/Game/Blueprints/Hori.Hori_C" (`KismetMathLibrary.MakeTransform` (0.0 0.0 0.0) (`KismetMathLibrary.MakeRotator` (`local.RotationX`))) "AlwaysSpawn" "OverrideRootScale" null (break `/Game/Blueprints/SceneSaver` _value) (`.Door?_7_F2A2430846CB07D8690779BDEF39561D` (break `/Game/Blueprints/SceneSaver` _value)) (`self.HideDoor?`) (`.DoorPos_22_6DC14774433C6D1F4A9ACB8BA6954658` (break `/Game/Blueprints/SceneSaver` _value)) (`.Y?_11_233DBD9B400006D0CEBCC2BFAE57E98C` (break `/Game/Blueprints/SceneSaver` _value)) (`.Furniture?_13_D5F072424BFB06945B0476BD17AC34A2` (break `/Game/Blueprints/SceneSaver` _value)) null)
          (else
            (if _returnvalue_2
              (set `local.tempDoor?` true)
              (else
                (set `local.tempDoor?` false)))
            (`|SpawnActorFromClass` "/Game/Blueprints/Hori.Hori_C" (`KismetMathLibrary.MakeTransform` (0.0 0.0 0.0) (`KismetMathLibrary.MakeRotator` (`local.RotationX`)) (1.0 1.0 -1.0)) "AlwaysSpawn" "OverrideRootScale" null (break `/Game/Blueprints/SceneSaver` _value) (`local.tempDoor?`) (`self.HideDoor?`) (`.DoorPos_22_6DC14774433C6D1F4A9ACB8BA6954658` (break `/Game/Blueprints/SceneSaver` _value_2)) (`.Y?_11_233DBD9B400006D0CEBCC2BFAE57E98C` (break `/Game/Blueprints/SceneSaver` _value)) (`.Furniture?_13_D5F072424BFB06945B0476BD17AC34A2` (break `/Game/Blueprints/SceneSaver` _value)) null)))))))

(fn `UserConstructionScript`
  (bind _doorcollision1 (`self.DoorCollision1`))
  (bind _doorcollision3 (`self.DoorCollision3`))
  (bind _doorcollision4 (`self.DoorCollision4`))
  (bind _doorcollision2 (`self.DoorCollision2`))
  (bind _returnvalue (/ (`self.Width`) 2.0))
  (bind _returnvalue_2 (/ (`self.DoorHeight`) 2.0))
  (bind _returnvalue_3 (/ (`self.DoorWidth`) 6.0))
  ;[1 1 1] DoorCollision Control
  (`|ExecutionSequence`
    (:`then_0`
      (`SceneComponent.K2_AddLocalOffset` (`self.C`) (`KismetMathLibrary.MakeVector` _returnvalue) false true)
      (`SceneComponent.K2_AddLocalOffset` (`self.D`) (`KismetMathLibrary.MakeVector` _returnvalue) false true)
      (`SceneComponent.K2_AddLocalOffset` (`self.A`) (`KismetMathLibrary.MakeVector` _returnvalue) false true)
      (`SceneComponent.K2_AddLocalOffset` (`self.B`) (`KismetMathLibrary.MakeVector` _returnvalue) false true))
    (:`then_1`
      (`BoxComponent.SetBoxExtent` _doorcollision1 (`KismetMathLibrary.MakeVector` _returnvalue_3 5.0 _returnvalue_2) true)
      (`SceneComponent.K2_SetRelativeLocation` _doorcollision1 (`KismetMathLibrary.MakeVector` (/ (`self.Width`) -3.0) -5.0 _returnvalue_2) false true)
      (`BoxComponent.SetBoxExtent` _doorcollision3 (`KismetMathLibrary.MakeVector` _returnvalue_3 5.0 _returnvalue_2) true)
      (`SceneComponent.K2_AddLocalOffset` _doorcollision3 (0.0 10.0 0.0) false true))
    (:`then_2`
      (`BoxComponent.SetBoxExtent` _doorcollision2 (`KismetMathLibrary.MakeVector` _returnvalue_3 5.0 _returnvalue_2) true)
      (`SceneComponent.K2_SetRelativeLocation` _doorcollision2 (`KismetMathLibrary.MakeVector` (/ (`self.Width`) 3.0) -5.0 _returnvalue_2) false true)
      (set `PrimitiveComponent.bGenerateOverlapEvents` false _doorcollision2)
      (`BoxComponent.SetBoxExtent` _doorcollision4 (`KismetMathLibrary.MakeVector` _returnvalue_3 5.0 _returnvalue_2) true)
      (`SceneComponent.K2_AddLocalOffset` _doorcollision4 (0.0 10.0 0.0) false true)
      (set `PrimitiveComponent.bGenerateOverlapEvents` false _doorcollision4))))