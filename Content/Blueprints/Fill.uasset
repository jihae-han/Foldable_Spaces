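; Procedural fill actor that dresses a box-sized area as a themed space (garden, city, office, meadow, Renaissance or grassland) in its construction script, chosen by Type.
; Helpers tile edge meshes with a stretched last piece, place corner props, build a procedural roof quad and randomly scatter ground meshes, optionally avoiding the doorway.
; Meshes are placed through instanced static mesh components created per call.
; Beyond is unfinished, with zeroed divisions and no instance locations.
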(fn `Beyond`
  (params (Mesh :type "StaticMesh Object Reference") (Density :type Integer) (Side :type String))
  (bind _returnvalue (* (`.ReturnValue` (`KismetMathLibrary.FMod` 0.0)) Density))
  (bind _returnvalue_2 (`AddComponent|NODE_AddInstancedStaticMeshComponent-10`))
  (`StaticMeshComponent.SetStaticMesh` _returnvalue_2 Mesh)
  (`|ExecutionSequence`
    (:`then_0`
      (if (`KismetStringLibrary.Contains` Side "1")
        (for _ (range 1 (+ (* Density (`.ReturnValue` (`KismetMathLibrary.FMod` 0.0))) 1))
          (`InstancedStaticMeshComponent.AddInstance` _returnvalue_2 (`KismetMathLibrary.MakeTransform` (0.0 0.0 0.0) (struct :`Yaw` 180.0))))))
    (:`then_1`
      (if (`KismetStringLibrary.Contains` Side "2")
        (for _ (range 1 (+ _returnvalue 1))
          (`InstancedStaticMeshComponent.AddInstance` _returnvalue_2 (`KismetMathLibrary.MakeTransform` (0.0 0.0 0.0) (struct :`Yaw` 90.0))))))
    (:`then_2`
      (if (`KismetStringLibrary.Contains` Side "3")
        (for _ (range 1 (+ _returnvalue 1))
          (`InstancedStaticMeshComponent.AddInstance` _returnvalue_2 (`KismetMathLibrary.MakeTransform` (0.0 0.0 0.0) (struct :`Yaw` 180.0))))))))

(fn `BorderMesh`
  (params (Mesh :type "StaticMesh Object Reference"))
  (locals (LengthX :type Integer) (LengthY :type Integer) (Location :type "Vector Structure") (ScaleX :type "Float (double-precision)") (ScaleY :type "Float (double-precision)") (Scale :type "Float (double-precision)" :default 1.05) (MeshExtentX :type "Float (double-precision)"))
  (bind _meshextentx (`local.MeshExtentX`))
  (bind _lengthx (`local.LengthX`))
  (bind _lengthy (`local.LengthY`))
  (bind _meshextentx_2 (`local.MeshExtentX`))
  (bind _meshextentx_3 (`local.MeshExtentX`))
  (bind _lengthx_2 (`local.LengthX`))
  (bind (_boxextent_x _boxextent_y) (`KismetMathLibrary.BreakVector` (`BoxComponent.BoxExtent` (`self.BoxExtent`))))
  (bind (_boxextent_x_2 _boxextent_y_2) (`KismetMathLibrary.BreakVector` (`BoxComponent.BoxExtent` (`self.BoxExtent`))))
  (bind (_boxextent_x_3 _boxextent_y_3) (`KismetMathLibrary.BreakVector` (`BoxComponent.BoxExtent` (`self.BoxExtent`))))
  (bind (_remainder _returnvalue) (`KismetMathLibrary.FMod` (* _boxextent_x 2.0) _meshextentx))
  (bind (_remainder_2 _returnvalue_2) (`KismetMathLibrary.FMod` (* _boxextent_y 2.0) _meshextentx))
  (bind _returnvalue_3 (`AddComponent|NODE_AddInstancedStaticMeshComponent-3`))
  (`StaticMeshComponent.SetStaticMesh` _returnvalue_3 Mesh)
  (set `local.MeshExtentX` (* (.x (`.BoxExtent` (`KismetMathLibrary.BreakBoxSphereBounds` (`StaticMesh.GetBounds` Mesh)))) 2.0))
  (`|ExecutionSequence`
    (:`then_0`
      (set `local.LengthX` _returnvalue_2)
      (if (< _remainder_2 (* _meshextentx 0.35))
        (set `local.ScaleX` (/ (+ _meshextentx_3 _remainder_2 10.0) _meshextentx_3))
        (else
          (set `local.ScaleX` (/ _remainder_2 _meshextentx_3))
          (`/Engine/EditorBlueprintResources/StandardMacros.IncrementInt` (`local.LengthX`)))))
    (:`then_1`
      (set `local.LengthY` _returnvalue)
      (if (< _remainder (* _meshextentx 0.35))
        (set `local.ScaleY` (/ (+ _remainder _meshextentx_2 10.0) _meshextentx_2))
        (else
          (set `local.ScaleY` (/ _remainder _meshextentx_2))
          (`/Engine/EditorBlueprintResources/StandardMacros.IncrementInt` (`local.LengthY`)))))
    (:`then_2`
      (for _index (range 1 (+ _lengthx 1))
        (if (== _lengthx _index)
          (set `local.Scale` (`local.ScaleX`)))
        (`InstancedStaticMeshComponent.AddInstance` _returnvalue_3 (`KismetMathLibrary.MakeTransform` (`local.Location`) (struct :`Yaw` 90.0) (`KismetMathLibrary.MakeVector` (`local.Scale`) 1.0 1.0)))
        (set `local.Location` (+ (`local.Location`) (`KismetMathLibrary.MakeVector` 0.0 (`local.MeshExtentX`)))))
      (set `local.Location` (`KismetMathLibrary.MakeVector` 0.0 (* _boxextent_y_2 2.0)))
      (set `local.Scale` 1.05)
      (for _index_2 (range 1 (+ _lengthy 1))
        (if (== _index_2 _lengthy)
          (set `local.Scale` (`local.ScaleY`)))
        (`InstancedStaticMeshComponent.AddInstance` _returnvalue_3 (`KismetMathLibrary.MakeTransform` (`local.Location`) (struct) (`KismetMathLibrary.MakeVector` (`local.Scale`) 1.0 1.0)))
        (set `local.Location` (+ (`local.Location`) (`KismetMathLibrary.MakeVector` (`local.MeshExtentX`)))))
      (set `local.Location` (`KismetMathLibrary.MakeVector` (* _boxextent_x_3 2.0) (* _boxextent_y_3 2.0)))
      (set `local.Scale` 1.05)
      (for _index_3 (range 1 (+ _lengthx_2 1))
        (if (== _lengthx_2 _index_3)
          (set `local.Scale` (`local.ScaleX`)))
        (`InstancedStaticMeshComponent.AddInstance` _returnvalue_3 (`KismetMathLibrary.MakeTransform` (`local.Location`) (struct :`Yaw` -90.0) (`KismetMathLibrary.MakeVector` (`local.Scale`) 1.0 1.0)))
        (set `local.Location` (- (`local.Location`) (`KismetMathLibrary.MakeVector` 0.0 (`local.MeshExtentX`))))))))

(fn `BorderVariegated`
  (params (Mesh :type "StaticMesh Object Reference") (Mesh1 :type "StaticMesh Object Reference") (Mesh2 :type "StaticMesh Object Reference"))
  (locals (Count :type Integer) (LengthX :type Integer) (LengthY :type Integer) (Location :type "Vector Structure") (ScaleX :type "Float (double-precision)") (ScaleY :type "Float (double-precision)") (Scale :type "Float (double-precision)" :default 1.1))
  (`|ExecutionSequence`
    (:`then_0`
      (`self.BorderX` Mesh))
    (:`then_1`
      (`/Engine/EditorBlueprintResources/StandardMacros.IsValid` Mesh1
        (:`Is Valid`
          (`self.BorderY` Mesh1))
        (:`Is Not Valid`
          (`self.BorderY` Mesh))))
    (:`then_2`
      (`/Engine/EditorBlueprintResources/StandardMacros.IsValid` Mesh2
        (:`Is Valid`
          (`self.BorderX` Mesh2))
        (:`Is Not Valid`
          (`self.BorderX` Mesh))))))

(fn `BorderX`
  (params (Mesh :type "StaticMesh Object Reference") (OtherEdge :type Boolean) (StretchZ :type "Float (double-precision)" :default 1.0) (AnchorOffset :type Boolean :default false))
  (locals (LengthX :type Integer) (Location :type "Vector Structure") (ScaleX :type "Float (double-precision)") (Scale :type "Float (double-precision)" :default 1.01) (MeshExtentX :type "Float (double-precision)") (Rotation :type "Float (double-precision)" :default -90.0) (MeshExtentY :type "Float (double-precision)"))
  (bind _returnvalue (`StaticMesh.GetBounds` Mesh))
  (bind _meshextentx (`local.MeshExtentX`))
  (bind _meshextentx_2 (`local.MeshExtentX`))
  (bind _location (`local.Location`))
  (bind _lengthx (`local.LengthX`))
  (bind _returnvalue_2 (* (`local.MeshExtentX`) 0.5 (`local.ScaleX`)))
  (bind (_boxextent_x _boxextent_y) (`KismetMathLibrary.BreakVector` (`BoxComponent.BoxExtent` (`self.BoxExtent`))))
  (bind (_remainder _returnvalue_3) (`KismetMathLibrary.FMod` (* _boxextent_y 2.0) _meshextentx_2))
  (bind _returnvalue_4 (`AddComponent|NODE_AddInstancedStaticMeshComponent-8`))
  (`StaticMeshComponent.SetStaticMesh` _returnvalue_4 Mesh)
  (set `local.MeshExtentX` (* (.x (`.BoxExtent` (`KismetMathLibrary.BreakBoxSphereBounds` _returnvalue))) 2.0))
  (set `local.MeshExtentY` (.y (`.BoxExtent` (`KismetMathLibrary.BreakBoxSphereBounds` _returnvalue))))
  (if OtherEdge
    (set `local.Location` (`KismetMathLibrary.MakeVector` (* _boxextent_x 2.0) (.x (`.BoxExtent` (`KismetMathLibrary.BreakBoxSphereBounds` _returnvalue))))) ; Left Edge
    (set `local.Rotation` 90.0)
    (else
      (set `local.Location` (`KismetMathLibrary.MakeVector` (* -0.6 (.y (`.BoxExtent` (`KismetMathLibrary.BreakBoxSphereBounds` _returnvalue)))) (.x (`.BoxExtent` (`KismetMathLibrary.BreakBoxSphereBounds` _returnvalue))))) ; Right Edge
    ))
  (`|ExecutionSequence`
    (:`then_0`
      (set `local.LengthX` _returnvalue_3)
      (if (< _remainder (* _meshextentx_2 0.35))
        (set `local.ScaleX` (/ (+ _meshextentx _remainder 10.0) _meshextentx))
        (else
          (set `local.ScaleX` (/ _remainder _meshextentx))
          (`/Engine/EditorBlueprintResources/StandardMacros.IncrementInt` (`local.LengthX`)))))
    (:`then_1`
      (if (and OtherEdge AnchorOffset)
        (set `local.Location` (- _location (`KismetMathLibrary.MakeVector` 0.0 _returnvalue_2)))
        (elif AnchorOffset
          (set `local.Location` (+ _location (`KismetMathLibrary.MakeVector` 0.0 _returnvalue_2))))))
    (:`then_2`
      (for _index (range 1 (+ _lengthx 1))
        (if (== _lengthx _index)
          (bind _output_get (set `local.Scale` (`local.ScaleX`)))
          (set `local.Location` (+ (- (`local.Location`) (`KismetMathLibrary.MakeVector` 0.0 (/ (`local.MeshExtentX`) 2.0))) (`KismetMathLibrary.MakeVector` 0.0 (* (`local.MeshExtentX`) 0.5 _output_get)))))
        (`InstancedStaticMeshComponent.AddInstance` _returnvalue_4 (`KismetMathLibrary.MakeTransform` (`local.Location`) (`KismetMathLibrary.MakeRotator` 0.0 0.0 (`local.Rotation`)) (`KismetMathLibrary.MakeVector` (`local.Scale`) 1.0 StretchZ)))
        (set `local.Location` (+ (`local.Location`) (`KismetMathLibrary.MakeVector` 0.0 (`local.MeshExtentX`))))))))

(fn `BorderY`
  (params (Mesh :type "StaticMesh Object Reference") (NoStretch :type Boolean) (StretchZ :type "Float (double-precision)") (AnchorOffset :type Boolean))
  (locals (LengthY :type Integer) (Location :type "Vector Structure") (ScaleY :type "Float (double-precision)") (Scale :type "Float (double-precision)" :default 1.0) (MeshExtentX :type "Float (double-precision)"))
  (bind _meshextentx (`local.MeshExtentX`))
  (bind _meshextentx_2 (`local.MeshExtentX`))
  (bind _location_x (`KismetMathLibrary.BreakVector` (`local.Location`)))
  (bind _lengthy (`local.LengthY`))
  (bind (_boxextent_x _boxextent_y) (`KismetMathLibrary.BreakVector` (`BoxComponent.BoxExtent` (`self.BoxExtent`))))
  (bind (_boxextent_x_2 _boxextent_y_2) (`KismetMathLibrary.BreakVector` (`BoxComponent.BoxExtent` (`self.BoxExtent`))))
  (bind (_remainder _returnvalue) (`KismetMathLibrary.FMod` (* _boxextent_x_2 2.0) _meshextentx))
  (bind _returnvalue_2 (`AddComponent|NODE_AddInstancedStaticMeshComponent-9`))
  (`StaticMeshComponent.SetStaticMesh` _returnvalue_2 Mesh)
  (bind _returnvalue_3 (`StaticMesh.GetBounds` (`StaticMeshComponent.StaticMesh` _returnvalue_2)))
  (set `local.MeshExtentX` (* (.x (`.BoxExtent` (`KismetMathLibrary.BreakBoxSphereBounds` _returnvalue_3))) 2.0))
  (set `local.Location` (`KismetMathLibrary.MakeVector` (.x (`.BoxExtent` (`KismetMathLibrary.BreakBoxSphereBounds` _returnvalue_3))) (* _boxextent_y_2 2.0)))
  (`|ExecutionSequence`
    (:`then_0`
      (set `local.LengthY` _returnvalue)
      (if (< _remainder (* _meshextentx 0.35))
        (set `local.ScaleY` (/ (+ _remainder _meshextentx_2 0.0) _meshextentx_2))
        (else
          (set `local.ScaleY` (/ _remainder _meshextentx_2))
          (`/Engine/EditorBlueprintResources/StandardMacros.IncrementInt` (`local.LengthY`)))))
    (:`then_1`
      (if AnchorOffset
        (set `local.Location` (+ (`local.Location`) (`KismetMathLibrary.MakeVector` (* (`local.MeshExtentX`) 0.5 (`local.ScaleY`)))))))
    (:`then_2`
      (for _index (range 1 (+ _lengthy 1))
        (if (== _index _lengthy)
          (bind _output_get (set `local.Scale` (`local.ScaleY`)))
          (set `local.Location` (`KismetMathLibrary.MakeVector` (+ (- _location_x (/ (`local.MeshExtentX`) 2.0)) (* (`local.MeshExtentX`) 0.5 _output_get)) (* _boxextent_y 2.0))))
        (`InstancedStaticMeshComponent.AddInstance` _returnvalue_2 (`KismetMathLibrary.MakeTransform` (`local.Location`) (struct :`Yaw` 180.0) (`KismetMathLibrary.MakeVector` (`local.Scale`) 1.0 StretchZ)))
        (set `local.Location` (+ (`local.Location`) (`KismetMathLibrary.MakeVector` (`local.MeshExtentX`))))))))

(fn `Corner`
  (params (Mesh :type "StaticMesh Object Reference") (InitialRotation :type "Float (double-precision)") (Corners :type String) (Padding :type "Float (double-precision)") (SetHeight :type "Float (double-precision)" :default 1.0))
  (locals (InnerCorners :type "Map of Integer to Vector Structure") (Rotation :type "Float (double-precision)") (NewLocalVar_0 :type Boolean :default false))
  (bind _innercorners (`local.InnerCorners`))
  (bind (_boxextent_x _boxextent_y) (`KismetMathLibrary.BreakVector` (`BoxComponent.BoxExtent` (`self.BoxExtent`))))
  (bind _returnvalue (`AddComponent|NODE_AddInstancedStaticMeshComponent-12`))
  (`StaticMeshComponent.SetStaticMesh` _returnvalue Mesh)
  (set `local.Rotation` InitialRotation)
  (`|ExecutionSequence`
    (:`then_0`
      (if (`KismetStringLibrary.Contains` Corners "0")
        (bind _returnvalue_2 (`StaticMesh.GetBounds` (`StaticMeshComponent.StaticMesh` _returnvalue)))
        (bind _returnvalue_3 (* (.x (`.BoxExtent` (`KismetMathLibrary.BreakBoxSphereBounds` _returnvalue_2))) Padding))
        (bind _returnvalue_4 (* (.y (`.BoxExtent` (`KismetMathLibrary.BreakBoxSphereBounds` _returnvalue_2))) Padding))
        (`BlueprintMapLibrary.Map_Add` _innercorners 0 (`KismetMathLibrary.MakeVector` _returnvalue_3 _returnvalue_4))))
    (:`then_1`
      (if (`KismetStringLibrary.Contains` Corners "1")
        (bind _returnvalue_5 (- (* _boxextent_y 2.0) _returnvalue_4))
        (`BlueprintMapLibrary.Map_Add` _innercorners 1 (`KismetMathLibrary.MakeVector` _returnvalue_3 _returnvalue_5))))
    (:`then_2`
      (if (`KismetStringLibrary.Contains` Corners "2")
        (bind _returnvalue_6 (- (* _boxextent_x 2.0) _returnvalue_3))
        (`BlueprintMapLibrary.Map_Add` _innercorners 2 (`KismetMathLibrary.MakeVector` _returnvalue_6 _returnvalue_5))))
    (:`then_3`
      (if (`KismetStringLibrary.Contains` Corners "3")
        (`BlueprintMapLibrary.Map_Add` _innercorners 3 (`KismetMathLibrary.MakeVector` _returnvalue_6))))
    (:`then_4`
      (for _index (range 4)
        (bind (_value _returnvalue_7) (`BlueprintMapLibrary.Map_Find` (`local.InnerCorners`) _index))
        (if _returnvalue_7
          (`InstancedStaticMeshComponent.AddInstance` _returnvalue (`KismetMathLibrary.MakeTransform` _value (`KismetMathLibrary.MakeRotator` 0.0 0.0 (`local.Rotation`)) (`KismetMathLibrary.MakeVector` 1.0 1.0 SetHeight)))
          (set `local.Rotation` (- (`local.Rotation`) 90.0)))))))

(fn `FillMesh`
  (params (Mesh :type "StaticMesh Object Reference") (Density :type "Float (double-precision)") (ZOffset :type "Float (double-precision)"))
  (locals (RandomX :type "Float (double-precision)") (RandomY :type "Float (double-precision)"))
  (bind (_returnvalue_min _returnvalue_max) (break `Box` (`StaticMesh.GetBoundingBox` Mesh)))
  (bind (_returnvalue_min_2 _returnvalue_max_2) (break `Box` (`StaticMesh.GetBoundingBox` Mesh)))
  (bind _doorleftpt (`self.DoorLeftPt`))
  (bind (_returnvalue_x _returnvalue_y) (`KismetMathLibrary.BreakVector` (/ _returnvalue_max 2)))
  (bind (_returnvalue_x_2 _returnvalue_y_2) (`KismetMathLibrary.BreakVector` (/ _returnvalue_max_2 2)))
  (bind (_boxextent_x _boxextent_y) (`KismetMathLibrary.BreakVector` (`BoxComponent.BoxExtent` (`self.BoxExtent`))))
  (bind _returnvalue (`AddComponent|NODE_AddInstancedStaticMeshComponent-1`))
  (`StaticMeshComponent.SetStaticMesh` _returnvalue Mesh)
  (for _ (range (+ (`KismetMathLibrary.FTrunc` (* (/ (+ _boxextent_x _boxextent_y) 50.0) Density)) 1))
    (bind _output_get (set `local.RandomX` (`KismetMathLibrary.RandomFloatInRange` _returnvalue_x (- (* _boxextent_x 2.0) _returnvalue_x))))
    (bind _output_get_2 (set `local.RandomY` (`KismetMathLibrary.RandomFloatInRange` _returnvalue_y (- (* _boxextent_y 2.0) _returnvalue_y))))
    (if (`self.NoDoor?`)
      (`InstancedStaticMeshComponent.AddInstance` _returnvalue (`KismetMathLibrary.MakeTransform` (`KismetMathLibrary.MakeVector` (`local.RandomX`) (`local.RandomY`) ZOffset)) :!label _label)
      (elif (not (and (`KismetMathLibrary.InRange_FloatFloat` _output_get (- _doorleftpt _returnvalue_x_2) (+ (`self.DoorWidth`) _doorleftpt _returnvalue_x_2) false false) (`KismetMathLibrary.InRange_FloatFloat` _output_get_2 0.0 (+ (`self.DoorHeight`) _returnvalue_y_2) false false)))
        (goto _label)))))

(fn `Roof`
  (params (Material :type "Material Object Reference") (Height :type "Float (double-precision)"))
  (bind (_returnvalue_x _returnvalue_y) (`KismetMathLibrary.BreakVector` (* (`BoxComponent.BoxExtent` (`self.BoxExtent`)) 2.0)))
  (bind _returnvalue (`AddComponent|NODE_AddProceduralMeshComponent-0` :`RelativeTransform` (`KismetMathLibrary.MakeTransform` (`KismetMathLibrary.MakeVector` 0.0 0.0 (- Height 10.0)))))
  (`ProceduralMeshComponent.CreateMeshSection_LinearColor` :`self` _returnvalue :`Vertices` (`|MakeArray` (0.0 0.0 0.0) (`KismetMathLibrary.MakeVector` 0.0 _returnvalue_y) (`KismetMathLibrary.MakeVector` _returnvalue_x _returnvalue_y) (`KismetMathLibrary.MakeVector` _returnvalue_x) :!type "Vector Structure") :`Triangles` (`|MakeArray` 0 2 1 0 3 2) :`UV0` (`|MakeArray` (0.0 0.0) (0.0 1.0) (1.0 1.0) (1.0 0.0) :!type "Vector2D Structure") :`bCreateCollision` true)
  (`PrimitiveComponent.SetMaterial` _returnvalue 0 Material))

(fn `UserConstructionScript`
  (bind _2nddoor (`self.2ndDoor`))
  (switch `/Game/Blueprints/PageEnum` (`self.Type`)
    (:`NewEnumerator5`
      ;[1 1 1] Garden
      (`|ExecutionSequence`
        (:`then_0`
          (if (> _2nddoor 0)
            (`self.BorderY` "/Game/Border/SM_Metal_Fence1_Short.SM_Metal_Fence1_Short" false 1.0 true)
            (if (> _2nddoor 1)
              (`self.BorderX` "/Game/Border/SM_Metal_Fence1_Short.SM_Metal_Fence1_Short" true 1.0 true)
              (else
                (`self.BorderX` "/Game/Border/SM_Metal_Fence1_Short.SM_Metal_Fence1_Short" false 1.0 true)))
            (else
              (`self.BorderMesh` "/Game/Border/SM_Metal_Fence1_Short.SM_Metal_Fence1_Short"))))
        (:`then_1`
          (`self.Corner` "/Game/Border/SM_Metal_Pillar2.SM_Metal_Pillar2" 45.0 "12" 1.0 0.87)
          (`self.Roof` "/Game/Floor/M_Wood_Floor_Walnut_Polished.M_Wood_Floor_Walnut_Polished" 270.0)
          (`self.Corner` "/Game/Corner/SM_Classic_chair.SM_Classic_chair" 135.0 "2" 2.0))
        (:`then_2`
          (`self.FillMesh` "/Game/Corner/SM_MERGED_heartLeaf.SM_MERGED_heartLeaf" 0.1)
          (`self.FillMesh` "/Game/Corner/SM_MERGED_cactus.SM_MERGED_cactus" 0.1)
          (`self.FillMesh` "/Game/Corner/SM_MERGED_peaceLily.SM_MERGED_peaceLily" 0.15)
          (`self.FillMesh` "/Game/Corner/SM_MERGED_cannaFlower.SM_MERGED_cannaFlower" 0.1)
          (`self.FillMesh` "/Game/Corner/SM_MERGED_heartLeafLarge.SM_MERGED_heartLeafLarge" 0.1)
          (`self.FillMesh` "/Game/Corner/SM_MERGED_philodendron.SM_MERGED_philodendron" 0.1)
          (`self.FillMesh` "/Game/Corner/SM_MERGED_snakePlant.SM_MERGED_snakePlant" 0.1))))
    (:`NewEnumerator6`
      ;[1 1 1] City
      (`self.BorderX` "/Game/Border/SM_Window_Frame_With_Glass1.SM_Window_Frame_With_Glass1")
      (`self.BorderX` "/Game/Border/SM_Window_Frame_With_Glass1.SM_Window_Frame_With_Glass1" true)
      (`self.BorderY` "/Game/Border/SM_Wall_Medium2.SM_Wall_Medium2" false 0.68)
      (`self.Roof` "/Game/Floor/M_Wood_Floor_Walnut_Polished.M_Wood_Floor_Walnut_Polished" 270.0)
      (`self.Corner` "/Game/Corner/SM_MERGED_philodendron.SM_MERGED_philodendron" 0.0 "2" 1.0)
      (`self.Corner` "/Game/Beyond/SM_Poplar_plant_B_00.SM_Poplar_plant_B_00" 0.0 "23" -0.7))
    (:`NewEnumerator4`
      ;[1 1 1] Office
      (`|ExecutionSequence`
        (:`then_0`
          (`self.BorderX` "/Game/Border/SM_Window.SM_Window" false 1.5)
          (`self.BorderY` "/Game/Border/SM_Window.SM_Window" false 1.5)
          (`self.BorderX` "/Game/Border/SM_Window.SM_Window" true 1.5)
          (`self.Roof` "/Game/Floor/M_Basic_Wall.M_Basic_Wall" 280.0))
        (:`then_1`
          (`self.Corner` "/Game/Corner/SM_ExecutiveChair.SM_ExecutiveChair" 135.0 "2" 2.0))))
    (:`NewEnumerator2`
      ;[1 1 1] Meadows
      (`|ExecutionSequence`
        (:`then_1`
          (`self.FillMesh` "/Game/Corner/SM_grass_meadow_06.SM_grass_meadow_06" 1.0)
          (`self.FillMesh` "/Game/Corner/SM_flower_chamomile_01_cross.SM_flower_chamomile_01_cross" 0.5)
          (`self.FillMesh` "/Game/Corner/SM_flower_common_poppy_01_cross.SM_flower_common_poppy_01_cross" 0.4)
          (`self.FillMesh` "/Game/Corner/SM_flower_goldenrod_02_cross.SM_flower_goldenrod_02_cross" 0.2)
          (`self.FillMesh` "/Game/Corner/SM_maple_bush_01.SM_maple_bush_01" 0.2))))
    (:`NewEnumerator1`
      ;[1 1 1] Renaissance
      (`|ExecutionSequence`
        (:`then_0`
          (`self.BorderX` "/Game/Border/SM_Wall_High_Sec1_Window1_Bottom.SM_Wall_High_Sec1_Window1_Bottom")
          (`self.BorderY` "/Game/Border/SM_Wall_High_Sec1_Window2_Upper_Ext.SM_Wall_High_Sec1_Window2_Upper_Ext" false 1.0)
          (`self.BorderX` "/Game/Border/SM_Wall_Pannel1.SM_Wall_Pannel1" true))
        (:`then_1`
          (`self.Beyond` "/Game/Beyond/SM_Poplar_tree_05_Optimised.SM_Poplar_tree_05_Optimised" 1 "13"))))
    (:`NewEnumerator0`
      ;[1 1 1] Grassland
      (`|ExecutionSequence`
        (:`then_0`
          (`self.BorderMesh` "/Game/Border/SM_wood_fence_type_04_B.SM_wood_fence_type_04_B"))
        (:`then_1`
          (`self.FillMesh` "/Game/Fill/SM_Grass_01.SM_Grass_01" 1.5 5.0)
          (`self.FillMesh` "/Game/Fill/SM_Grass_02.SM_Grass_02" 0.4 3.0)
          (`self.FillMesh` "/Game/Fill/SM_Grass_07.SM_Grass_07" 0.3 3.0)
          (`self.FillMesh` "/Game/Fill/SM_Grass_07.SM_Grass_07" 0.2 3.0))))))