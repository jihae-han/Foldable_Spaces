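; Actor Blueprint that builds a flat procedural square and swaps its geometry when the mesh is hit.
; The construction script creates a colliding 100-unit quad in the XY plane with a chrome metal material.
; The first component hit sets the Change flag and recreates the section from the Vertices, Triangles and UV variables, without requesting collision.
; Any hit received while Change is set only prints a debug message.
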(event `self.ProceduralMesh.OnComponentHit`
  (params (HitComponent :type "PrimitiveComponent Object Reference") (OtherActor :type "Actor Object Reference") (OtherComp :type "PrimitiveComponent Object Reference") (NormalImpulse :type "Vector Structure") (Hit :type "HitResult Structure (by ref)"))
  (if (`self.change`)
    (`KismetSystemLibrary.PrintString` "Change has occured")
    (else
      (set `self.change` true)
      (`ProceduralMeshComponent.CreateMeshSection_LinearColor` :`self` (`self.ProceduralMesh`) :`Vertices` (`self.vertices`) :`Triangles` (`self.triangles`) :`UV0` (`self.UV`)))))

(fn `UserConstructionScript`
  (bind _proceduralmesh (`self.ProceduralMesh`))
  (`ProceduralMeshComponent.CreateMeshSection_LinearColor` :`self` _proceduralmesh :`Vertices` (`|MakeArray` (0.0 0.0 0.0) (0.0 100.0 0.0) (100.0 100.0 0.0) (100.0 0.0 0.0) :!type "Vector Structure") :`Triangles` (`|MakeArray` 0 1 2 0 2 3) :`UV0` (`|MakeArray` (0.0 0.0) (0.0 1.0) (1.0 1.0) (1.0 0.0) :!type "Vector2D Structure") :`bCreateCollision` true)
  (`PrimitiveComponent.SetMaterial` _proceduralmesh 0 "/Game/StarterContent/Materials/M_Metal_Chrome.M_Metal_Chrome"))