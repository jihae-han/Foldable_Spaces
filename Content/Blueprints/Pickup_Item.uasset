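; Pickup item actor that displays a configurable mesh with an offset box component; no pickup logic exists yet, as its event graph is empty.
; The construction script adds an instanced static mesh component, assigns the Mesh variable and creates a single instance at the origin.
; It then shifts the Box by the X and Z offset variables.
; Nodes for sizing the box from mesh bounds and setting its collision are left disconnected.
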(fn `UserConstructionScript`
  (bind _returnvalue (`AddComponent|NODE_AddInstancedStaticMeshComponent-0`))
  (`StaticMeshComponent.SetStaticMesh` _returnvalue (`self.Mesh`))
  (`InstancedStaticMeshComponent.AddInstance` _returnvalue (`KismetMathLibrary.MakeTransform` (0.0 0.0 0.0) (struct) (1.0 1.0 1.0)))
  (`SceneComponent.K2_AddLocalOffset` (`self.Box`) (`KismetMathLibrary.MakeVector` (`self.X-Offset`) 0.0 (`self.Z-Offset`)) false true))