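; Dragon is a skeletal mesh actor that can be picked up and dropped.
; Pickup turns off mesh physics and attaches the root to the given component, while Drop re-enables physics and detaches the actor, both tracking a PickedUp flag.
; Separately, any Box overlap attaches the skeletal mesh to the overlapping component in place, without checking that flag or changing physics.
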(event `self.Box.OnComponentBeginOverlap`
  (params (OverlappedComponent :type "PrimitiveComponent Object Reference") (OtherActor :type "Actor Object Reference") (OtherComp :type "PrimitiveComponent Object Reference") (OtherBodyIndex :type Integer) (bFromSweep :type Boolean) (SweepResult :type "HitResult Structure (by ref)"))
  (`SceneComponent.K2_AttachToComponent` (`self.SkeletalMeshComponent`) OtherComp "None" "KeepWorld" "KeepWorld" "KeepWorld" false))

(event `/Game/Blueprints/PickupActorInterface.Pickup`
  (params (AttachTo :type "SceneComponent Object Reference"))
  (`PrimitiveComponent.SetSimulatePhysics` (`self.SkeletalMeshComponent`) false)
  (`SceneComponent.K2_AttachToComponent` (`self.RootComponent`) AttachTo "None" "KeepWorld" "KeepWorld" "KeepWorld" false)
  (set `self.PickedUp` true))

(event `/Game/Blueprints/PickupActorInterface.Drop`
  (`PrimitiveComponent.SetSimulatePhysics` (`self.SkeletalMeshComponent`) true)
  (`self.K2_DetachFromActor` "KeepWorld" "KeepWorld" "KeepWorld")
  (set `self.PickedUp` false))

(fn `UserConstructionScript`)